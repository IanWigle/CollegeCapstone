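; AI-controlled turret that hands its active weapon's ability to its AI for firing.
; Shortly after BeginPlay it writes that ability class and a CanFire flag to the AI controller's Blackboard, then caches a self reference.
; Tick and the construction script are empty, and a base-rotation sound node is left unconnected.
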(event EventBeginPlay
  (Utilities|FlowControl|Delay 0.2)
  (bind _asaicontroller (Utilities|Casting|CastToAIController (Pawn|GetController)))
  (Class|BlackboardComponent|SetValueasClass (AI|GetBlackboard _asaicontroller) (Utilities|Name|MakeLiteralName "CurrentWeaponAbility") (Variables|/Script/Outpost_Production.BaseWeapon|Getm_WeaponAbility (Variables|Default|Getm_ActiveTurretWeapon)))
  (AI|Components|Blackboard|SetValueasBool (AI|GetBlackboard _asaicontroller) (Utilities|Name|MakeLiteralName "CanFire") true)
  (bind _asbp_turret (Utilities|Casting|CastToBP_Turret self))
  (Variables|Default|SetSelfRef _asbp_turret))

(event EventTick
  (params (DeltaSeconds :type Float%20%28single-precision%29)))

(fn ConstructionScript)