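; BP_DrillObjective is a drill objective actor that plays its running sound at the mesh location while the objective is active.
; Tick checks IsObjectiveActive and uses a six-second Delay, which ignores retriggers while pending, to replay the loop cue periodically.
; A timed intro sequence of falling, artillery and startup cues is disconnected and never runs, and SignalThatObjectiveHasStarted is empty.
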(event EventSignalThatObjectiveHasStarted)

(event EventTick
  (params (DeltaSeconds :type Float%20%28single-precision%29))
  (bind _returnvalue (Class|DrillObjective|IsObjectiveActive))
  (if _returnvalue
    (Utilities|FlowControl|Delay 6.0)
    (Audio|PlaySoundatLocation "/Game/Assets/Sound/FX/Drill/Drill_Running_Loop_Cue.Drill_Running_Loop_Cue" (Transformation|GetWorldLocation (Variables|Character|GetMesh)) "0, 0, 0" 1.0 1.0 0.0 "/Game/Blueprints/Audio/BP_EffectAttenuation.BP_EffectAttenuation" 0 0)))

(fn ConstructionScript)