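; Player mech Blueprint that handles HUD, audio, boost effect, death feedback and tutorial progression.
; BeginPlay creates the HUD, applies the sound mix, fixes post-process brightness bounds and, for the local player, hooks looping music after the intro track.
; Gameplay events advance tutorial steps for firing, reloading, base use and turret repair, zeroing turret repair cost and signalling player readiness.
; Death plays a randomly chosen sound and directional animation, picked independently.
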(event Custom|StartBoost
  (bind _boost (Variables|Default|GetBoost))
  (Components|Activation|Deactivate _boost)
  (Components|Activation|Activate _boost false))

(event Custom|Server_Boost
  (CallFunction|StartBoost))

(event Custom|MusicLoop
  (Audio|PlaySoundatLocation "/Game/Assets/Sound/Music/Music/InGame_Loop_Cue.InGame_Loop_Cue" "0, 0, 0" "0, 0, 0" 1.0 1.0 0.0 0 0 0))

(event Custom|OnDeathEvent_1
  (bind _death_right_am (Variables|Default|GetDeath%20Right%20AM))
  (bind _death_left_am (Variables|Default|GetDeath%20Left%20AM))
  (bind _death1_sc (Variables|Default|GetDeath1%20SC))
  (bind _death1_sc_2 (Variables|Default|GetDeath1%20SC))
  (bind _death4_sc (Variables|Default|GetDeath4%20SC))
  (bind _death3_sc (Variables|Default|GetDeath3%20SC))
  (bind _death_forward_am (Variables|Default|GetDeath%20Forward%20AM))
  (bind _death_back_am (Variables|Default|GetDeath%20Back%20AM))
  (bind _array (Utilities|Array|MakeArray _death_forward_am _death_back_am _death_right_am _death_left_am))
  (bind _array_2 (Utilities|Array|MakeArray _death1_sc _death1_sc_2 _death3_sc _death4_sc))
  (Audio|PlaySoundatLocation (Utilities|Array|Get(acopy) _array_2 (Math|Random|RandomIntegerinRange 0 (- (Utilities|Array|Length _array_2) 1))) (Transformation|GetActorLocation (Variables|Default|GetSelfRef)) "0, 0, 0" 1.0 1.0 0.0 0 0 0)
  (Components|Animation|PlayAnimation (Variables|Character|GetMesh) (Utilities|Array|Get(acopy) _array (Math|Random|RandomIntegerinRange 0 (- (Utilities|Array|Length _array) 1))) false))

(event EventBeginPlay
  (bind _returnvalue (UserInterface|CreateWidget "/Game/Blueprints/Entities/Player/HUD/Widget_HUD.Widget_HUD_C"))
  (UserInterface|Viewport|AddtoViewport _returnvalue 0)
  (CallFunction|UpdateBrightness 1.0)
  (Class|GameplayStatics|SetBaseSoundMix "/Game/Assets/Audio/GameSoundMix.GameSoundMix")
  (bind _asbp_player_mech (Utilities|Casting|CastToBP_PlayerMech self))
  (Variables|Default|SetSelfRef _asbp_player_mech)
  (if (Pawn|IsLocallyControlled)
    (EventDispatchers|BindEventtoOnAudioFinished (Variables|Default|GetInGameMusic) (delegate Custom|MusicLoop))))

(event EventOnEventPlayerFiredLeftWeapon
  (Class|PlayerMech|ClientAdvanceTutorial 1 -1.0))

(event EventOnEventPlayerFiredRightWeapon
  (Class|PlayerMech|ClientAdvanceTutorial 1 -1.0))

(event EventDisplayWinWidget
  (bind _returnvalue (UserInterface|CreateWidget "/Game/Blueprints/Entities/Player/HUD/WinGameMenu.WinGameMenu_C"))
  (UserInterface|Viewport|AddtoViewport _returnvalue 0))

(event EventOnEventPlayerRepairedTurrets
  (Class|PlayerMech|ServerPlayerIsReady)
  (Class|PlayerMech|ClientAdvanceTutorial 5 -1.0)
  (Variables|/Script/Outpost_Production.Turret|Setm_TurretRepairCost (Variables|Default|Getm_Turret) 0))

(event EventOnEventPlayerFiredSpecial
  (Class|PlayerMech|ClientAdvanceTutorial 3 -1.0))

(event EventOnEventFirstBaseInteract
  (Class|PlayerMech|ClientAdvanceTutorial 4 -1.0))

(event EventOnEventFirstReload
  (Class|PlayerMech|ClientAdvanceTutorial 2 -1.0))

(event EventOnEventPlayerPlacedTurret
  (bind _m_turret (Variables|Default|Getm_Turret))
  (Variables|Default|SetOriginalTurretRepairCost (Variables|/Script/Outpost_Production.Turret|Getm_TurretRepairCost _m_turret))
  (Variables|/Script/Outpost_Production.Turret|Setm_TurretRepairCost _m_turret 0)
  (Audio|PlaySoundatLocation "/Game/Assets/Sound/FX/TurretBase/TurretBase_Deploy_Cue.TurretBase_Deploy_Cue" (Transformation|GetActorLocation _m_turret) "0, 0, 0" 1.0 1.0 0.0 0 0 0))

(fn ConstructionScript)

(fn UpdateBrightness
  (params (NewBrightness :type Float%20%28single-precision%29))
  (bind _outactors (Actor|GetAllActorsOfClass "/Script/Engine.PostProcessVolume"))
  (for _array_element _outactors
    (Variables|/Script/Engine.PostProcessVolume|SetSettings _array_element (Utilities|Struct|MakePostProcessSettings NewBrightness NewBrightness))))