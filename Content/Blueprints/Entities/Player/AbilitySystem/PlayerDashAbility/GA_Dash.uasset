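; GA_Dash is the player mech's dash Gameplay Ability, propelling BP_PlayerMech along its forward vector.
; After a successful commit, it ends early if the mech is dead, otherwise calls ServerBoost, plays a boost sound and fires start and loop montages back to back.
; A timed root motion constant force with a strength curve drives movement and clamps exit velocity, then the end montage plays and the ability ends.
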(event Ability|EventActivateAbility
  (bind _returnvalue (Ability|GetAvatarActorfromActorInfo))
  (bind _returnvalue_2 (Ability|CommitAbility))
  (if _returnvalue_2
    (bind _asbp_player_mech (Utilities|Casting|CastToBP_PlayerMech (Ability|GetOwningActorfromActorInfo)))
    (if (Variables|/Script/Outpost_Production.BaseEntity|Getm_bIsDead _asbp_player_mech)
      (Ability|EndAbility)
      (else
        (Default|ServerBoost _asbp_player_mech)
        (Animation|PlayAnimMontage _asbp_player_mech (Variables|/Game/Blueprints/Entities/Player/BP_PlayerMech.BP_PlayerMech_C|GetDash%20Start%20AM _asbp_player_mech) 1.0 "None")
        (Audio|PlaySoundatLocation "/Game/Assets/Sound/FX/Mech/Mech_Boost_Cue.Mech_Boost_Cue" (Transformation|GetActorLocation _returnvalue) "0, 0, 0" 1.0 1.0 0.0 0 0 0)
        (Animation|PlayAnimMontage _asbp_player_mech (Variables|/Game/Blueprints/Entities/Player/BP_PlayerMech.BP_PlayerMech_C|GetDash%20Loop%20AM _asbp_player_mech) 1.0 "None")
        (Ability|Tasks|ApplyRootMotionConstantForce "None" (Transformation|GetActorForwardVector _returnvalue) (Variables|Default|GetDashStrength) 0.75 false "/Game/Blueprints/Entities/Player/AbilitySystem/PlayerDashAbility/DashStrengthOverTime.DashStrengthOverTime" "ClampVelocity" (Transformation|GetVelocity _returnvalue)
          (:OnFinish
            (bind _asbp_player_mech_2 (Utilities|Casting|CastToBP_PlayerMech (Ability|GetOwningActorfromActorInfo)))
            (Animation|PlayAnimMontage _asbp_player_mech_2 (Variables|/Game/Blueprints/Entities/Player/BP_PlayerMech.BP_PlayerMech_C|GetDash%20End%20AM _asbp_player_mech_2) 1.0 "None")
            (Ability|EndAbility)))))
    (else
      (Ability|CancelAbility))))