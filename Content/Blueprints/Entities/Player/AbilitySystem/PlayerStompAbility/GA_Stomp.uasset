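; Gameplay ability for the player mech's stomp, an area attack that damages, stuns and knocks back nearby enemies.
; On activation it plays the stomp montage, and on blend out sphere-overlaps BaseEnemy actors around the avatar.
; Each enemy receives a SetByCaller damage effect and a stun-tag effect, then a slightly lifted radial impulse away from the player.
; EndAbility is called inside the enemy loop as well as after it.
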(event Ability|EventActivateAbility
  (bind _returnvalue (Ability|GetOwningActorfromActorInfo))
  (bind _asbp_player_mech (Utilities|Casting|CastToBP_PlayerMech (Ability|GetOwningActorfromActorInfo)))
  (Animation|Montage|PlayMontage (Variables|/Script/Engine.Character|GetMesh _asbp_player_mech) (Variables|/Game/Blueprints/Entities/Player/BP_PlayerMech.BP_PlayerMech_C|GetStomp%20AM _asbp_player_mech)
    (:OnBlendOut
      (bind _outactors (Collision|SphereOverlapActors (Transformation|GetActorLocation (Ability|GetAvatarActorfromActorInfo)) (Variables|Default|GetStompRange) (Utilities|Array|MakeArray "ObjectTypeQuery8") "/Script/Outpost_Production.BaseEnemy"))
      (for _array_element _outactors
        (bind _asbase_enemy (Utilities|Casting|CastToBaseEnemy _array_element))
        (Utilities|Casting|CastToBP_PlayerMech _returnvalue)
        (bind _returnvalue_2 (Ability|GameplayEffect|AssignTagSetbyCallerMagnitude (Ability|MakeOutgoingGameplayEffectSpec "/Game/Blueprints/Weapons/GE_Damage.GE_Damage_C") "(TagName=\"Damage\")" -1.0))
        (GameplayEffects|ApplyGameplayEffectSpecToSelf (Variables|/Script/Outpost_Production.BaseEntity|Getm_EntityAbilitySystemComponent _asbase_enemy) _returnvalue_2)
        (GameplayEffects|ApplyGameplayEffectToSelf :self (Variables|/Script/Outpost_Production.BaseEntity|Getm_EntityAbilitySystemComponent _asbase_enemy) :GameplayEffectClass "/Game/Blueprints/Entities/Player/AbilitySystem/PlayerStompAbility/GE_StompStunTag.GE_StompStunTag_C" :Level 1.0)
        (Class|NavMovementComponent|StopActiveMovement (Variables|/Script/Engine.Character|GetCharacterMovement _asbase_enemy))
        (Physics|AddImpulse (Variables|/Script/Engine.Character|GetCharacterMovement _asbase_enemy) (* (Math|Vector|MakeVector (.X (Math|Vector|BreakVector (Math|Vector|GetUnitDirection(Vector) (Transformation|GetActorLocation _returnvalue) (Transformation|GetActorLocation _asbase_enemy)))) (.Y (Math|Vector|BreakVector (Math|Vector|GetUnitDirection(Vector) (Transformation|GetActorLocation _returnvalue) (Transformation|GetActorLocation _asbase_enemy)))) 0.1) (Variables|Default|GetStompStrength)) true)
        (Ability|EndAbility))
      (Ability|EndAbility))))