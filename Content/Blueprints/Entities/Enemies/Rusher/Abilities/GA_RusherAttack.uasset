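; GA_RusherAttack is the Rusher enemy's attack gameplay ability, pairing a random charge or jump montage with a short AI move.
; As the montage starts, it saves the enemy's location and moves toward its scaled forward vector, used directly as a world position.
; Without waiting for that move, it commits and applies GE_RusherAttack to the blackboard Target's ability system.
; When the move finishes, it sends the enemy back without pathfinding and ends.
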(event Ability|EventActivateAbility
  (bind _attackcharge (Variables|Default|GetAttackCharge))
  (bind _attackjump (Variables|Default|GetAttackJump))
  (bind _array (Utilities|Array|MakeArray _attackcharge _attackjump))
  (bind _asbase_enemy (Utilities|Casting|CastToBaseEnemy (Ability|GetOwningActorfromActorInfo))
    (:then
      (Animation|Montage|PlayMontage (Variables|/Script/Engine.Character|GetMesh _asbase_enemy) (Utilities|Array|Get(acopy) _array (Math|Random|RandomIntegerinRange 0 (- (Utilities|Array|Length _array) 1)))
        (:then
          (bind _output_get (Variables|Default|SetStarting%20Location (Transformation|GetActorLocation _asbase_enemy)))
          (AI|AIMoveTo (AI|GetAIController _asbase_enemy) (* (Transformation|GetActorForwardVector _asbase_enemy) 5e+01) 0 -1.0 "Default" "Default" true true
            (:then
              (bind _asbase_entity (Utilities|Casting|CastToBaseEntity (AI|Components|Blackboard|GetValueasObject (AI|GetBlackboard _asbase_enemy) (Utilities|Name|MakeLiteralName "Target")))
                (:then
                  (Ability|CommitAbility)
                  (GameplayEffects|ApplyGameplayEffectToSelf :self (Ability|GetAbilitySystemComponent _asbase_entity) :GameplayEffectClass "/Game/Blueprints/Entities/Enemies/Rusher/Effects/GE_RusherAttack.GE_RusherAttack_C" :Level 1.0))
                (:CastFailed
                  (Development|PrintString "GA_RusherAttack - Target not BaseEntity! This is a problem" true true "(R=1.000000,G=0.059521,B=0.043605,A=1.000000)"))))
            (:OnMoveFinished
              (AI|Navigation|MovetoLocation (AI|GetAIController _asbase_enemy) _output_get 1.0 true false false true 0)
              (Ability|EndAbility))))))
    (:CastFailed
      (Ability|EndAbility))))