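; BP_Rusher is the Rusher enemy character Blueprint, handling animation and sound reactions to stun, falling, landing and death.
; Tick checks the ability system for the Entity.Stunned tag, triggering a cry and random stun montage, otherwise fall feedback while airborne, re-triggered every frame without a guard.
; Landing plays an impact sound and montage.
; The death event plays a random, non-looping death animation directly on the mesh.
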(event Custom|OnDeathEvent_1
  (bind _deathlight (Variables|Default|GetDeathLight))
  (bind _deathmed (Variables|Default|GetDeathMed))
  (bind _deathheavy (Variables|Default|GetDeathHeavy))
  (bind _array (Utilities|Array|MakeArray _deathlight _deathmed _deathheavy))
  (Components|Animation|PlayAnimation (Variables|Character|GetMesh) (Utilities|Array|Get(acopy) _array (Math|Random|RandomIntegerinRange 0 (- (Utilities|Array|Length _array) 1))) false))

(event EventBeginPlay
  (bind _asbp_rusher (Utilities|Casting|CastToBP_Rusher self))
  (Variables|Default|SetSelfRef _asbp_rusher))

(event Collision|EventActorBeginOverlap
  (params (OtherActor :type Actor%20Object%20Reference)))

(event EventTick
  (params (DeltaSeconds :type Float%20%28single-precision%29))
  (bind _stunlight (Variables|Default|GetStunLight))
  (bind _stunheavy (Variables|Default|GetStunHeavy))
  (bind _array (Utilities|Array|MakeArray _stunlight _stunheavy))
  (if (GameplayTags|HasMatchingGameplayTag (Variables|Default|Getm_EntityAbilitySystemComponent) "(TagName=\"Entity.Stunned\")")
    (Audio|SpawnSoundatLocation "/Game/Assets/Sound/FX/Rusher/Rusher_Cry_Cue.Rusher_Cry_Cue" (Transformation|GetActorLocation) "0, 0, 0" 1.0 1.0 0.0 "/Game/Blueprints/Audio/BP_EffectAttenuation.BP_EffectAttenuation" 0)
    (Animation|PlayAnimMontage (Utilities|Array|Get(acopy) _array (Math|Random|RandomIntegerinRange 0 (- (Utilities|Array|Length _array) 1))) 1.0 "None")
    (elif (AI|Components|NavMovement|IsFalling (Variables|Character|GetCharacterMovement))
      (Audio|PlaySoundatLocation "/Game/Assets/Sound/FX/Rusher/Rusher_Fall_Cue.Rusher_Fall_Cue" (Transformation|GetActorLocation) "0, 0, 0" 1.0 1.0 0.0 "/Game/Blueprints/Audio/BP_EffectAttenuation.BP_EffectAttenuation" 0 0)
      (Animation|PlayAnimMontage "/Game/Assets/3D_Assets/Enemies/Rusher/Actions/AM_Rusher_Falling.AM_Rusher_Falling" 1.0 "None"))))

(event EventOnLanded
  (params (Hit :type Hit%20Result%20Structure%20%28by%20ref%29))
  (Audio|PlaySoundatLocation "/Game/Assets/Sound/FX/Rusher/Rusher_FootImpact_Cue.Rusher_FootImpact_Cue" (Transformation|GetActorLocation) "0, 0, 0" 1.0 1.0 0.0 "/Game/Blueprints/Audio/BP_EffectAttenuation.BP_EffectAttenuation" 0 0)
  (Animation|PlayAnimMontage (Variables|Default|GetSelfRef) "/Game/Assets/3D_Assets/Enemies/Rusher/Actions/AM_Rusher_Landing.AM_Rusher_Landing" 1.0 "None"))

(fn ConstructionScript)