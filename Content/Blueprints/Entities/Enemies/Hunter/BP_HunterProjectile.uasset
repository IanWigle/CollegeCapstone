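; BP_HunterProjectile is the projectile owned by the Hunter enemy, delivering its damage through a gameplay event.
; Actor and collision-component overlaps share one path, which requires the owner to be a BP_Hunter.
; That path sets homing on the Hunter's current target only at overlap, then sends the Hunter a Damage event targeting the overlapped actor.
; The projectile then immediately destroys itself and prints a debug message.
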(event OnComponentBeginOverlap(HunterProjCollision)
  (params (OverlappedComponent :type Primitive%20Component%20Object%20Reference) (OtherActor :type Actor%20Object%20Reference) (OtherComp :type Primitive%20Component%20Object%20Reference) (OtherBodyIndex :type Integer) (bFromSweep :type Boolean) (SweepResult :type Hit%20Result%20Structure%20%28by%20ref%29))
  (bind _m_projectilemovement (Variables|Default|Getm_ProjectileMovement))
  (bind _asbp_hunter (Utilities|Casting|CastToBP_Hunter (Components|GetOwner)))
  (bind _returnvalue (Class|BaseEnemy|GetCurrentTarget _asbp_hunter))
  (bind _output_get (Variables|Default|SetTarget _returnvalue))
  (Variables|/Script/Engine.ProjectileMovementComponent|SetHomingTargetComponent _m_projectilemovement (Variables|/Script/Engine.Actor|GetRootComponent _output_get))
  (Variables|/Script/Engine.ProjectileMovementComponent|SetbIsHomingProjectile _m_projectilemovement true)
  (Ability|SendGameplayEventtoActor _asbp_hunter "(TagName=\"Damage\")" (Utilities|Struct|MakeGameplayEventData "" 0 OtherActor))
  (Actor|DestroyActor)
  (Development|PrintString "Hunter projectile destroyed"))

(event EventBeginPlay)

(event Collision|EventActorBeginOverlap
  (params (OtherActor :type Actor%20Object%20Reference))
  (bind _m_projectilemovement (Variables|Default|Getm_ProjectileMovement))
  (bind _asbp_hunter (Utilities|Casting|CastToBP_Hunter (Components|GetOwner)))
  (bind _returnvalue (Class|BaseEnemy|GetCurrentTarget _asbp_hunter))
  (bind _output_get (Variables|Default|SetTarget _returnvalue))
  (Variables|/Script/Engine.ProjectileMovementComponent|SetHomingTargetComponent _m_projectilemovement (Variables|/Script/Engine.Actor|GetRootComponent _output_get))
  (Variables|/Script/Engine.ProjectileMovementComponent|SetbIsHomingProjectile _m_projectilemovement true)
  (Ability|SendGameplayEventtoActor _asbp_hunter "(TagName=\"Damage\")" (Utilities|Struct|MakeGameplayEventData "" 0 (stale OnComponentBeginOverlap(HunterProjCollision) OtherActor)))
  (Actor|DestroyActor)
  (Development|PrintString "Hunter projectile destroyed"))

(event EventTick
  (params (DeltaSeconds :type Float%20%28single-precision%29)))

(fn ConstructionScript
  (Collision|SetActorEnableCollision true))