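; Gameplay ability for the Hunter enemy's ranged attack on its current target.
; On activation it commits, plays the attack montage and spawns BP_HunterProjectile at the attack-point socket, rotated from capsule facing toward the target via a single RInterpTo.
; It then waits for a Damage gameplay event, applies GE_HunterAttack to the payload target's ability system and ends.
; A failed Hunter cast or missing target ability system logs and ends it.
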(event Ability|EventActivateAbility
  (bind _ashunter (Utilities|Casting|CastToHunter (Ability|GetAvatarActorfromActorInfo))
    (:then
      ;[1 1 1] Make it always target the player
      (bind _returnvalue (Class|BaseEnemy|GetCurrentTarget _ashunter))
      (Variables|Default|SetTarget _returnvalue)
      (Ability|CommitAbility)
      (Animation|PlayAnimMontage _ashunter "/Game/Assets/3D_Assets/Enemies/Hunter/AnimMontage_Hunter_Attack.AnimMontage_Hunter_Attack" 1.0 "None")
      (Game|SpawnActorfromClass "/Game/Blueprints/Entities/Enemies/Hunter/BP_HunterProjectile.BP_HunterProjectile_C" (Math|Transform|MakeTransform (Transformation|GetSocketLocation (Variables|/Script/Engine.Character|GetMesh _ashunter) (Class|SkinnedMeshComponent|GetSocketBoneName (Variables|/Script/Engine.Character|GetMesh _ashunter) "Hunter_Attack_Point")) (Math|Interpolation|RInterpTo (Transformation|GetWorldRotation (Variables|/Script/Engine.Character|GetCapsuleComponent _ashunter)) (Math|Rotator|FindLookatRotation (Transformation|GetSocketLocation (Variables|/Script/Engine.Character|GetMesh _ashunter) (Class|SkinnedMeshComponent|GetSocketBoneName (Variables|/Script/Engine.Character|GetMesh _ashunter) "Hunter_Attack_Point")) (Transformation|GetActorLocation (Variables|Default|GetTarget))) (Utilities|Time|GetWorldDeltaSeconds) 1e+02)) "AlwaysSpawn" _ashunter 0)
      (bind _payload (Ability|Tasks|WaitGameplayEvent "(TagName=\"Damage\")" 0)
        (:EventReceived
          (Utilities|IsValid (Ability|GetAbilitySystemComponent (.Target (Utilities|Struct|BreakGameplayEventData _payload)))
            (:Is%20Valid
              (GameplayEffects|ApplyGameplayEffectSpecToSelf (Ability|GetAbilitySystemComponent (.Target (Utilities|Struct|BreakGameplayEventData _payload))) (Ability|MakeOutgoingGameplayEffectSpec "/Game/Blueprints/Entities/Enemies/Hunter/Effects/GE_HunterAttack.GE_HunterAttack_C"))
              (Ability|EndAbility))
            (:Is%20Not%20Valid
              ;[1 1 1] Fail States to end Ability
              (Development|PrintString "Target did not have ability system component")
              (Ability|EndAbility :!label _label))))))
    (:CastFailed
      (Development|PrintString "Failed to Cast as Hunter in GA hunter attack")
      (goto _label))))