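; Gameplay ability that makes the Hunter enemy dash forward along the ground plane.
; After committing, it plays the Hunter dodge montage and applies a constant root motion force along the capsule's flattened forward vector, keeping the last velocity on finish.
; The current target is fetched but does not affect the dash direction.
; The ability ends when the force finishes or the owner cast fails, and cancels if commit fails.
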(event Ability|EventActivateAbility
  (bind _returnvalue (Ability|CommitAbility))
  (if _returnvalue
    (bind _asbp_hunter (Utilities|Casting|CastToBP_Hunter (Ability|GetOwningActorfromActorInfo))
      (:then
        (Class|BaseEnemy|GetCurrentTarget _asbp_hunter)
        (Animation|PlayAnimMontage _asbp_hunter "/Game/Assets/3D_Assets/Enemies/Hunter/AnimMontage_Hunter_Dodge.AnimMontage_Hunter_Dodge" 1.0 "None")
        (Ability|Tasks|ApplyRootMotionConstantForce "None" (* (Math|Vector|GetForwardVector (Variables|/Script/Engine.Character|GetCapsuleComponent _asbp_hunter)) "1.000000,1.000000, 0") 2.5e+03 1.0 false 0 "MaintainLastRootMotionVelocity"
          (:OnFinish
            (Ability|EndAbility))))
      (:CastFailed
        (Ability|EndAbility)))
    (else
      (Ability|CancelAbility))))