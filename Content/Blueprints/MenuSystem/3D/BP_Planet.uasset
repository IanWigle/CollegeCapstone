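; BP_Planet is a planet actor for the 3D menu system that spins continuously.
; The construction script creates a dynamic instance of PlanetMaterial, passes PlanetRotationSpeed to its RotationSpeed parameter and applies it to the Planet component.
; Each Tick adds world yaw to Planet at that same speed scaled by delta seconds, so one variable drives both mesh and material.
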(event EventTick
  (params (DeltaSeconds :type Float%20%28single-precision%29))
  (Transformation|AddWorldRotation (Variables|Default|GetPlanet) (Math|Rotator|MakeRotator 0.0 0.0 (* (Variables|Default|GetPlanetRotationSpeed) (Utilities|Time|GetWorldDeltaSeconds))) false false))

(fn ConstructionScript
  (bind _returnvalue (Rendering|Material|CreateDynamicMaterialInstance (Variables|Default|GetPlanetMaterial) "None" :!class /Script/Engine.KismetMaterialLibrary))
  (Rendering|Material|SetScalarParameterValue _returnvalue "RotationSpeed" (Variables|Default|GetPlanetRotationSpeed) :!class /Script/Engine.MaterialInstanceDynamic)
  (Rendering|Material|SetMaterial (Variables|Default|GetPlanet) 0 _returnvalue))