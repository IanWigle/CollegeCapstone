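; Gameplay ability that fires the Old Reliable hitscan weapon for either a player mech or a turret.
; Mechs refire on a looping fire-rate timer, tracing from the camera until input release or failed ammo check.
; Turrets fire one shot per activation, tracing from the weapon to their blackboard target.
; Hits on Enemy-tagged actors apply GE_Damage via SetByCaller, with linear range falloff computed from weapon attributes.
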(event Custom|Refire_Event_Mech
  (bind _returnvalue (Ability|MakeOutgoingGameplayEffectSpec "/Game/Blueprints/Weapons/GE_Damage.GE_Damage_C"))
  (bind _playermech (Variables|Default|GetPlayerMech))
  (bind _weaponabilitysystem (Variables|Default|GetWeaponAbilitySystem))
  (bind _returnvalue_2 (Ability|Attribute|GetFloatAttributefromAbilitySystemComponent _weaponabilitysystem "(AttributeName=\"\",Attribute=StructProperty'\"/Script/Outpost_Production.BaseWeaponAttributeSet:m_SoftRange\"',AttributeOwner=None)"))
  (bind _returnvalue_3 (Ability|Attribute|GetFloatAttributefromAbilitySystemComponent _weaponabilitysystem "(AttributeName=\"\",Attribute=StructProperty'\"/Script/Outpost_Production.BaseWeaponAttributeSet:m_Damage\"',AttributeOwner=None)"))
  (bind _m_followcamera (Variables|/Script/Outpost_Production.PlayerMech|Getm_FollowCamera _playermech))
  (bind _returnvalue_4 (Transformation|GetWorldLocation _m_followcamera))
  (bind _returnvalue_5 (* _returnvalue_3 -1.0))
  ;[1 1 1] Ensure that we have ammo remaining to fire the gun
  (bind _returnvalue_6 (Class|GameplayAbility|CheckAbilityCost))
  (if _returnvalue_6
    (Ability|CommitAbilityCost false)
    (Class|BaseWeapon|NetMulticastWeaponFireStarted (Variables|Default|GetBaseWeapon))
    (bind (_outhit _returnvalue_7) (Collision|LineTraceByChannel _returnvalue_4 (+ _returnvalue_4 (* (Math|Vector|GetForwardVector _m_followcamera) (.ReturnValue (Ability|Attribute|GetFloatAttributefromAbilitySystemComponent (Variables|Default|GetWeaponAbilitySystem) "(AttributeName=\"\",Attribute=StructProperty'\"/Script/Outpost_Production.BaseWeaponAttributeSet:m_HardRange\"',AttributeOwner=None)")))) "TraceTypeQuery3" false (Utilities|Array|MakeArray _playermech (Variables|Default|GetBaseWeapon)) "ForDuration"))
    ;[1 1 1] Ensure we actually hit something
    (if _returnvalue_7
      (if (.bBlockingHit (Collision|BreakHitResult _outhit))
        (Utilities|IsValid (.HitActor (Collision|BreakHitResult _outhit))
          (:Is%20Valid
            (if (Actor|ActorHasTag (.HitActor (Collision|BreakHitResult _outhit)) "Enemy")
              (bind _asbase_entity (Utilities|Casting|CastToBaseEntity (.HitActor (Collision|BreakHitResult _outhit))))
              (Class|BaseWeapon|NetMulticastWeaponHit (Variables|Default|GetBaseWeapon) (.Location (Collision|BreakHitResult _outhit)) (.HitActor (Collision|BreakHitResult _outhit)))
              ;[1 1 1] Use different damage calc depending on if the target is in falloff range or not
              (if (>= (.Distance (Collision|BreakHitResult _outhit)) _returnvalue_2)
                (bind _returnvalue_8 (Ability|GameplayEffect|AssignTagSetbyCallerMagnitude _returnvalue "(TagName=\"Damage\")" (* _returnvalue_5 (- 1.0 (/ (- (.Distance (Collision|BreakHitResult _outhit)) _returnvalue_2) (- (.ReturnValue (Ability|Attribute|GetFloatAttributefromAbilitySystemComponent _weaponabilitysystem "(AttributeName=\"\",Attribute=StructProperty'\"/Script/Outpost_Production.BaseWeaponAttributeSet:m_HardRange\"',AttributeOwner=None)")) _returnvalue_2))))))
                (GameplayEffects|ApplyGameplayEffectSpecToSelf (Ability|GetAbilitySystemComponent _asbase_entity) _returnvalue_8)
                (else
                  (bind _returnvalue_9 (Ability|GameplayEffect|AssignTagSetbyCallerMagnitude _returnvalue "(TagName=\"Damage\")" _returnvalue_5))
                  (GameplayEffects|ApplyGameplayEffectSpecToSelf (Ability|GetAbilitySystemComponent _asbase_entity) _returnvalue_9))))))))
    (else
      (Ability|EndAbility))))

(event Ability|EventActivateAbility
  (bind _returnvalue (Ability|GetOwningActorfromActorInfo))
  (bind _asbp_base_weapon (Utilities|Casting|CastToBP_BaseWeapon (Ability|GetAvatarActorfromActorInfo)))
  (bind _output_get (Variables|Default|SetBaseWeapon _asbp_base_weapon))
  (Variables|Default|SetWeaponAbilitySystem (Ability|GetAbilitySystemComponent _output_get))
  (bind _asbp_player_mech (Utilities|Casting|CastToBP_PlayerMech _returnvalue)
    (:then
      (Variables|Default|SetPlayerMech _asbp_player_mech)
      ;[1 1 1] Waits for InputReleased event, when recieved, quit the gameplay ability
      (Ability|Tasks|WaitGameplayEvent "(TagName=\"Weapon.InputReleased\")" 0
        (:then
          (Utilities|Time|SetTimerbyEvent (delegate Custom|Refire_Event_Mech) (/ 6e+01 (.ReturnValue (Ability|Attribute|GetFloatAttributefromAbilitySystemComponent (Variables|Default|GetWeaponAbilitySystem) "(AttributeName=\"\",Attribute=StructProperty'\"/Script/Outpost_Production.BaseWeaponAttributeSet:m_FireRate\"',AttributeOwner=None)"))) true))
        (:EventReceived
          (Variables|Default|SetIsInputDown false)
          (Ability|EndAbility))))
    (:CastFailed
      (bind _asbp_turret (Utilities|Casting|CastToBP_Turret _returnvalue)
        (:then
          (Variables|TurretData|SetPlayerTurret _asbp_turret)
          (Ability|CommitAbilityCost false)
          (bind _asbase_weapon (Utilities|Casting|CastToBaseWeapon (Ability|GetCurrentSourceObject))
            (:then
              (Effects|SpawnEmitterAttached "/Game/Assets/VFX/ParticleSystems/PS_MuzzFlashSimple.PS_MuzzFlashSimple" (Variables|/Script/Engine.SkeletalMeshActor|GetSkeletalMeshComponent _asbase_weapon) "Muzzle_Socket_Top" "0, 0, 0" "0, 0, 0" "1.000000,1.000000,1.000000" "SnapToTarget" true "AutoRelease")
              (bind _asactor (Utilities|Casting|CastToActor (AI|Components|Blackboard|GetValueasObject (AI|GetBlackboard (Variables|TurretData|GetPlayerTurret)) (Utilities|Name|MakeLiteralName "CurrentTarget")))
                (:then
                  (bind _outhit (Collision|LineTraceByChannel (Transformation|GetWorldLocation (Variables|/Script/Engine.Actor|GetRootComponent (Variables|Default|GetBaseWeapon))) (Transformation|GetActorLocation _asactor) "TraceTypeQuery3" false (Utilities|Array|MakeArray (Variables|TurretData|GetPlayerTurret) (Variables|Default|GetBaseWeapon)) "ForDuration"))
                  (if (.bBlockingHit (Collision|BreakHitResult _outhit))
                    (Niagara|SpawnSystematLocation "/Game/Blueprints/Weapons/MainWeapons/OldReliable/TestEmitter_System.TestEmitter_System" (.Location (Collision|BreakHitResult _outhit)))
                    (Utilities|IsValid (.HitActor (Collision|BreakHitResult _outhit))
                      (:Is%20Valid
                        (if (Actor|ActorHasTag (.HitActor (Collision|BreakHitResult _outhit)) "Enemy")
                          (bind _asbase_entity (Utilities|Casting|CastToBaseEntity (.HitActor (Collision|BreakHitResult _outhit))))
                          (if (>= (.Distance (Collision|BreakHitResult _outhit)) (.ReturnValue (Ability|Attribute|GetFloatAttributefromAbilitySystemComponent (Ability|GetAbilitySystemComponent (Variables|Default|GetBaseWeapon)) "(AttributeName=\"\",Attribute=StructProperty'\"/Script/Outpost_Production.BaseWeaponAttributeSet:m_SoftRange\"',AttributeOwner=None)")))
                            (bind _returnvalue_2 (Ability|GameplayEffect|AssignTagSetbyCallerMagnitude (Ability|MakeOutgoingGameplayEffectSpec "/Game/Blueprints/Weapons/GE_Damage.GE_Damage_C") "(TagName=\"Damage\")" (* (- 1.0 (/ (- (.Distance (Collision|BreakHitResult _outhit)) (.ReturnValue (Ability|Attribute|GetFloatAttributefromAbilitySystemComponent (Ability|GetAbilitySystemComponent (Variables|Default|GetBaseWeapon)) "(AttributeName=\"\",Attribute=StructProperty'\"/Script/Outpost_Production.BaseWeaponAttributeSet:m_SoftRange\"',AttributeOwner=None)"))) (- (.ReturnValue (Ability|Attribute|GetFloatAttributefromAbilitySystemComponent (Ability|GetAbilitySystemComponent (Variables|Default|GetBaseWeapon)) "(AttributeName=\"\",Attribute=StructProperty'\"/Script/Outpost_Production.BaseWeaponAttributeSet:m_HardRange\"',AttributeOwner=None)")) (.ReturnValue (Ability|Attribute|GetFloatAttributefromAbilitySystemComponent (Ability|GetAbilitySystemComponent (Variables|Default|GetBaseWeapon)) "(AttributeName=\"\",Attribute=StructProperty'\"/Script/Outpost_Production.BaseWeaponAttributeSet:m_SoftRange\"',AttributeOwner=None)"))))) (* (.ReturnValue (Ability|Attribute|GetFloatAttributefromAbilitySystemComponent (Ability|GetAbilitySystemComponent (Variables|Default|GetBaseWeapon)) "(AttributeName=\"\",Attribute=StructProperty'\"/Script/Outpost_Production.BaseWeaponAttributeSet:m_Damage\"',AttributeOwner=None)")) -1.0))))
                            (GameplayEffects|ApplyGameplayEffectSpecToSelf (Ability|GetAbilitySystemComponent _asbase_entity) _returnvalue_2)
                            (Development|PrintString (Utilities|String|ToString(Float) (* (- 1.0 (/ (- (.Distance (Collision|BreakHitResult _outhit)) (.ReturnValue (Ability|Attribute|GetFloatAttributefromAbilitySystemComponent (Ability|GetAbilitySystemComponent (Variables|Default|GetBaseWeapon)) "(AttributeName=\"\",Attribute=StructProperty'\"/Script/Outpost_Production.BaseWeaponAttributeSet:m_SoftRange\"',AttributeOwner=None)"))) (- (.ReturnValue (Ability|Attribute|GetFloatAttributefromAbilitySystemComponent (Ability|GetAbilitySystemComponent (Variables|Default|GetBaseWeapon)) "(AttributeName=\"\",Attribute=StructProperty'\"/Script/Outpost_Production.BaseWeaponAttributeSet:m_HardRange\"',AttributeOwner=None)")) (.ReturnValue (Ability|Attribute|GetFloatAttributefromAbilitySystemComponent (Ability|GetAbilitySystemComponent (Variables|Default|GetBaseWeapon)) "(AttributeName=\"\",Attribute=StructProperty'\"/Script/Outpost_Production.BaseWeaponAttributeSet:m_SoftRange\"',AttributeOwner=None)"))))) (* (.ReturnValue (Ability|Attribute|GetFloatAttributefromAbilitySystemComponent (Ability|GetAbilitySystemComponent (Variables|Default|GetBaseWeapon)) "(AttributeName=\"\",Attribute=StructProperty'\"/Script/Outpost_Production.BaseWeaponAttributeSet:m_Damage\"',AttributeOwner=None)")) -1.0))))
                            (else
                              (bind _returnvalue_3 (Ability|GameplayEffect|AssignTagSetbyCallerMagnitude (Ability|MakeOutgoingGameplayEffectSpec "/Game/Blueprints/Weapons/GE_Damage.GE_Damage_C") "(TagName=\"Damage\")" (* (.ReturnValue (Ability|Attribute|GetFloatAttributefromAbilitySystemComponent (Ability|GetAbilitySystemComponent (Variables|Default|GetBaseWeapon)) "(AttributeName=\"\",Attribute=StructProperty'\"/Script/Outpost_Production.BaseWeaponAttributeSet:m_Damage\"',AttributeOwner=None)")) -1.0)))
                              (GameplayEffects|ApplyGameplayEffectSpecToSelf (Ability|GetAbilitySystemComponent _asbase_entity) _returnvalue_3)
                              (Development|PrintString "no falloff")))
                          (Ability|EndAbility)
                          (else
                            (Ability|EndAbility :!label _label))))
                      (:Is%20Not%20Valid
                        (goto _label)))
                    (else
                      (goto _label))))
                (:CastFailed
                  (Ability|EndAbility))))
            (:CastFailed
              (Ability|EndAbility))))
        (:CastFailed
          (Ability|EndAbility))))))

(event Ability|EventOnEndAbility
  (params (bWasCancelled :type Boolean))
  (Class|BaseWeapon|NetMulticastWeaponStopFire (Variables|Default|GetBaseWeapon)))