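; Old Reliable, a mech main weapon that handles firing presentation and initializes its GAS attributes and tags from a data table and gameplay effect.
; Each shot plays a montage, sustains firing audio, and alternates muzzle flash and Niagara bullet trail between top and bottom barrels.
; Trails aim from the muzzle toward a far point along the player's camera forward.
; Hits spawn pooled blood or dust by Enemy tag; stopping plays an end sound.
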(event EventBeginPlay
  (bind _m_weaponabilitysystemcomponent (Variables|Default|Getm_WeaponAbilitySystemComponent))
  (Class|AbilitySystemComponent|InitStats _m_weaponabilitysystemcomponent "/Script/Outpost_Production.BaseWeaponAttributeSet" "/Game/Blueprints/Weapons/MainWeapons/OldReliable/OldReliableDataTable.OldReliableDataTable")
  (GameplayEffects|ApplyGameplayEffectToSelf :self _m_weaponabilitysystemcomponent :GameplayEffectClass "/Game/Blueprints/Weapons/MainWeapons/OldReliable/GE_Old_Reliable_Tags.GE_Old_Reliable_Tags_C"))

(event EventWeaponFireEvent
  (bind _m_audiocomponent (Variables|Default|Getm_AudioComponent))
  (bind _skeletalmeshcomponent (Variables|Default|GetSkeletalMeshComponent))
  (bind _returnvalue (Math|Vector|GetRightVector _skeletalmeshcomponent))
  (Animation|Montage|PlayMontage (Variables|Default|GetSkeletalMeshComponent) "/Game/Assets/3D_Assets/Character/Weapons/Ol_Reliable/SK_OlReliable_Fire_Montage.SK_OlReliable_Fire_Montage"
    (:then
      (if (Audio|Components|Audio|IsPlaying _m_audiocomponent)
        _
        (else
          (Audio|Components|Audio|Play _m_audiocomponent 0.0)))
      (if (Variables|Default|GetHasFiredTop)
        (Components|Activation|Activate (Variables|Default|GetNS_BottomFlash) true)
        (Variables|Default|SetHasFiredTop false)
        (Niagara|SetNiagaraVariable(Vector3) (Variables|Default|GetNS_BottomFlash) "User.Direction" _returnvalue)
        (CallFunction|ActivateBulletTrail "Muzzle_Socket_Bottom")
        (else
          (Components|Activation|Activate (Variables|Default|GetNS_TopFlash) true)
          (Variables|Default|SetHasFiredTop true)
          (Niagara|SetNiagaraVariable(Vector3) (Variables|Default|GetNS_TopFlash) "User.Direction" _returnvalue)
          (CallFunction|ActivateBulletTrail "Muzzle_Socket_Top"))))))

(event EventWeaponHitEvent
  (params (endLocation :type Vector :default "0, 0, 0") (hitActor :type Actor%20Object%20Reference))
  (Utilities|IsValid hitActor
    (:Is%20Valid
      (if (Actor|ActorHasTag hitActor "Enemy")
        (Niagara|SpawnSystematLocation "/Game/Assets/VFX/ParticleSystems/WeaponHitEffects/HitEnemy/NS_BloodSplatter.NS_BloodSplatter" endLocation "0, 0, 0" "1.000000,1.000000,1.000000" true true "AutoRelease")
        (else
          (Niagara|SpawnSystematLocation "/Game/Assets/VFX/ParticleSystems/WeaponHitEffects/DustHit/NS_DustHIt.NS_DustHIt" endLocation "0, 0, 0" "1.000000,1.000000,1.000000" true true "AutoRelease"))))))

(event EventWeaponStopFireEvent
  (Audio|PlaySoundatLocation "/Game/Assets/Sound/FX/Weapons/Ol_ReliableEnd_Cue.Ol_ReliableEnd_Cue" (Transformation|GetActorLocation) "0, 0, 0" 1.0 1.0 0.0 0 0 0)
  (Audio|Components|Audio|Stop (Variables|Default|Getm_AudioComponent)))

(fn ConstructionScript)

(fn ActivateBulletTrail
  (params (InSocketName :type Name))
  (bind _skeletalmeshcomponent (Variables|Default|GetSkeletalMeshComponent))
  (bind _returnvalue (Transformation|GetSocketLocation _skeletalmeshcomponent InSocketName))
  (bind _asplayer_mech (Utilities|Casting|CastToPlayerMech (Components|GetOwner)))
  (bind _returnvalue_2 (Niagara|SpawnSystematLocation "/Game/Assets/VFX/ParticleSystems/BulletTrace/NS_BulletTrail.NS_BulletTrail" _returnvalue))
  (Niagara|SetNiagaraVariable(Vector3) _returnvalue_2 "User.DirectionVector" (Math|Vector|Normalize (- (+ (* (Math|Vector|GetForwardVector (Variables|/Script/Outpost_Production.PlayerMech|Getm_FollowCamera _asplayer_mech)) 5000) (Transformation|GetWorldLocation (Variables|/Script/Outpost_Production.PlayerMech|Getm_FollowCamera _asplayer_mech))) _returnvalue)))
  (Niagara|SetNiagaraVariable(Vector3) _returnvalue_2 "User.FacingVector" (Math|Vector|GetRightVector _skeletalmeshcomponent)))