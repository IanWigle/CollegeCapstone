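; Gameplay ability that fires a multi-pellet hitscan shotgun for a player mech or turret.
; The mech traces random cone-spread pellets from its camera, while a turret traces straight at its blackboard CurrentTarget.
; FirePellet spawns blood or dust particles and applies GE_Damage to Enemy-tagged entities, reduced linearly beyond a falloff range.
; Attributes drive the stats, and GE_Reload is applied inside the pellet loop with a fire-rate-based SetByCaller magnitude.
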(event Ability|EventActivateAbility
  (bind _returnvalue (Ability|GetOwningActorfromActorInfo))
  (bind _asbase_weapon (Utilities|Casting|CastToBaseWeapon (Ability|GetAvatarActorfromActorInfo))
    (:then
      (Variables|Default|SetWeapon _asbase_weapon)
      (Variables|Default|SetAbilitySystem (Ability|GetAbilitySystemComponent _asbase_weapon))
      (Ability|CommitAbility)
      (if false
        (Ability|EndAbility :!label _label)
        (else
          (bind _asplayer_mech (Utilities|Casting|CastToPlayerMech _returnvalue)
            (:then
              (if (.bSuccessfullyFoundAttribute (Ability|Attribute|GetFloatAttributefromAbilitySystemComponent (Variables|Default|GetAbilitySystem) "(AttributeName=\"\",Attribute=StructProperty'\"/Script/Outpost_Production.BaseWeaponAttributeSet:m_HardRange\"',AttributeOwner=None)"))
                (Class|BaseWeapon|NetMulticastWeaponFireStarted (Variables|Default|GetWeapon))
                (for _index (range 0 (Variables|Default|GetNumberOfPellets))
                  (CallFunction|FirePellet (Transformation|GetWorldLocation (Variables|/Script/Outpost_Production.PlayerMech|Getm_FollowCamera _asplayer_mech)) (+ (* (Math|Random|RandomUnitVectorinConeinDegrees (Math|Vector|GetForwardVector (Variables|/Script/Outpost_Production.PlayerMech|Getm_FollowCamera _asplayer_mech)) (.ReturnValue (Ability|Attribute|GetFloatAttributefromAbilitySystemComponent (Variables|Default|GetAbilitySystem) "(AttributeName=\"\",Attribute=StructProperty'\"/Script/Outpost_Production.BaseWeaponAttributeSet:m_Spread\"',AttributeOwner=None)"))) (.ReturnValue (Ability|Attribute|GetFloatAttributefromAbilitySystemComponent (Variables|Default|GetAbilitySystem) "(AttributeName=\"\",Attribute=StructProperty'\"/Script/Outpost_Production.BaseWeaponAttributeSet:m_HardRange\"',AttributeOwner=None)"))) (Transformation|GetWorldLocation (Variables|/Script/Outpost_Production.PlayerMech|Getm_FollowCamera _asplayer_mech))) (Variables|Default|GetAbilitySystem) (Utilities|Array|MakeArray (Variables|Default|GetWeapon) _asplayer_mech))
                  (bind _returnvalue_2 (Ability|GameplayEffect|AssignTagSetbyCallerMagnitude (Ability|MakeOutgoingGameplayEffectSpec "/Game/Blueprints/Weapons/MainWeapons/GE_Reload.GE_Reload_C") "(TagName=\"Weapon.Reloading\")" (/ 6e+01 (.ReturnValue (Ability|Attribute|GetFloatAttribute (Variables|Default|GetWeapon) "(AttributeName=\"\",Attribute=StructProperty'\"/Script/Outpost_Production.BaseWeaponAttributeSet:m_FireRate\"',AttributeOwner=None)")))))
                  (GameplayEffects|ApplyGameplayEffectSpecToSelf (Variables|Default|GetAbilitySystem) _returnvalue_2))
                (Development|PrintString (Utilities|String|Append "Shotgun CurrentAmmo: " (Utilities|String|ToString(Float) (.ReturnValue (Ability|Attribute|GetFloatAttribute (Variables|Default|GetWeapon) "(AttributeName=\"m_CurrentAmmo\",Attribute=StructProperty'\"/Script/Outpost_Production.BaseWeaponAttributeSet:m_CurrentAmmo\"',AttributeOwner=Class'\"/Script/Outpost_Production.BaseWeaponAttributeSet\"')")))))
                (Ability|EndAbility)
                (else
                  (Development|PrintString "GA_ShotgunRevised - Failed to find HardRange"))))
            (:CastFailed
              (bind _asturret (Utilities|Casting|CastToTurret _returnvalue)
                (:then
                  (bind _asactor (Utilities|Casting|CastToActor (AI|Components|Blackboard|GetValueasObject (AI|GetBlackboard _asturret) (Utilities|Name|MakeLiteralName "CurrentTarget")))
                    (:then
                      (Class|BaseWeapon|NetMulticastWeaponFireStarted (Variables|Default|GetWeapon))
                      (for _index_2 (range 0 (Variables|Default|GetNumberOfPellets))
                        (CallFunction|FirePellet (Transformation|GetActorLocation _asturret) (Transformation|GetActorLocation _asactor) (Variables|Default|GetAbilitySystem) (Utilities|Array|MakeArray _asturret (Variables|Default|GetWeapon)))
                        (bind _returnvalue_3 (Ability|GameplayEffect|AssignTagSetbyCallerMagnitude (Ability|MakeOutgoingGameplayEffectSpec "/Game/Blueprints/Weapons/MainWeapons/GE_Reload.GE_Reload_C") "(TagName=\"Weapon.Reloading\")" (/ 6e+01 (.ReturnValue (Ability|Attribute|GetFloatAttribute (Variables|Default|GetWeapon) "(AttributeName=\"\",Attribute=StructProperty'\"/Script/Outpost_Production.BaseWeaponAttributeSet:m_FireRate\"',AttributeOwner=None)")))))
                        (GameplayEffects|ApplyGameplayEffectSpecToSelf (Variables|Default|GetAbilitySystem) _returnvalue_3))
                      (Ability|EndAbility))
                    (:CastFailed
                      (Ability|EndAbility))))
                (:CastFailed
                  (Ability|EndAbility))))))))
    (:CastFailed
      (Development|PrintString "GA_ShotgunRevised - Cast to BaseWeaponFailed")
      (goto _label))))

(fn FirePellet
  (params (Start :type Vector) (End :type Vector) (AbilityComponent :type Ability%20System%20Component%20Object%20Reference) (ActorsToIgnore :type Array%20of%20Actor%20Object%20References))
  (bind _returnvalue (Ability|Attribute|GetFloatAttributefromAbilitySystemComponent AbilityComponent "(AttributeName=\"\",Attribute=StructProperty'\"/Script/Outpost_Production.BaseWeaponAttributeSet:m_Damage\"',AttributeOwner=None)"))
  (bind _returnvalue_2 (Ability|Attribute|GetFloatAttributefromAbilitySystemComponent AbilityComponent "(AttributeName=\"\",Attribute=StructProperty'\"/Script/Outpost_Production.BaseWeaponAttributeSet:m_SoftRange\"',AttributeOwner=None)"))
  (bind _returnvalue_3 (* _returnvalue -1.0))
  (bind _outhit (Collision|LineTraceByChannel Start End "TraceTypeQuery3" false ActorsToIgnore "ForDuration"))
  (if (.bBlockingHit (Collision|BreakHitResult _outhit))
    (CallFunction|SpawnCorrectHitParticle (.HitActor (Collision|BreakHitResult _outhit)) (.Location (Collision|BreakHitResult _outhit)))
    (Utilities|IsValid (.HitActor (Collision|BreakHitResult _outhit))
      (:Is%20Valid
        (if (Actor|ActorHasTag (.HitActor (Collision|BreakHitResult _outhit)) "Enemy")
          (bind _asbase_entity (Utilities|Casting|CastToBaseEntity (.HitActor (Collision|BreakHitResult _outhit))))
          (if (>= (.Distance (Collision|BreakHitResult _outhit)) _returnvalue_2)
            (bind _returnvalue_4 (Ability|GameplayEffect|AssignTagSetbyCallerMagnitude (Ability|MakeOutgoingGameplayEffectSpec "/Game/Blueprints/Weapons/GE_Damage.GE_Damage_C") "(TagName=\"Damage\")" (* _returnvalue_3 (- 1.0 (/ (- (.Distance (Collision|BreakHitResult _outhit)) _returnvalue_2) (- (.ReturnValue (Ability|Attribute|GetFloatAttributefromAbilitySystemComponent AbilityComponent "(AttributeName=\"\",Attribute=StructProperty'\"/Script/Outpost_Production.BaseWeaponAttributeSet:m_HardRange\"',AttributeOwner=None)")) _returnvalue_2))))))
            (GameplayEffects|ApplyGameplayEffectSpecToSelf (Ability|GetAbilitySystemComponent _asbase_entity) _returnvalue_4)
            (else
              (bind _returnvalue_5 (Ability|GameplayEffect|AssignTagSetbyCallerMagnitude (Ability|MakeOutgoingGameplayEffectSpec "/Game/Blueprints/Weapons/GE_Damage.GE_Damage_C") "(TagName=\"Damage\")" _returnvalue_3))
              (GameplayEffects|ApplyGameplayEffectSpecToSelf (Ability|GetAbilitySystemComponent _asbase_entity) _returnvalue_5)))
          (Class|BaseWeapon|NetMulticastWeaponHit (Variables|Default|GetWeapon) (.Location (Collision|BreakHitResult _outhit)) (.HitActor (Collision|BreakHitResult _outhit))))))))

(fn SpawnCorrectHitParticle
  (params (HitActor :type Actor%20Object%20Reference) (HitLocation :type Vector))
  (Utilities|IsValid HitActor
    (:Is%20Valid
      (if (Actor|ActorHasTag HitActor "Enemy")
        (Niagara|SpawnSystematLocation "/Game/Assets/VFX/ParticleSystems/WeaponHitEffects/HitEnemy/NS_BloodSplatter.NS_BloodSplatter" HitLocation "0, 0, 0" "1.000000,1.000000,1.000000" true true "AutoRelease")
        (else
          (Niagara|SpawnSystematLocation "/Game/Assets/VFX/ParticleSystems/WeaponHitEffects/DustHit/NS_DustHIt.NS_DustHIt" HitLocation "0, 0, 0" "1.000000,1.000000,1.000000" true true "AutoRelease"))))))