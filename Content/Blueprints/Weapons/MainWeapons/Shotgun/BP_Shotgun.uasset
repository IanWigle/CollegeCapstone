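; Shotgun weapon Blueprint that sets up its Gameplay Ability System data and handles cosmetic feedback for firing and hits.
; BeginPlay initializes attributes from a shotgun data table and applies a tag GameplayEffect to its own ability system component.
; Fire events play the montage, sound and Niagara muzzle flash.
; Hit events spawn a bullet trail aimed from the muzzle socket, plus blood for Enemy-tagged actors or dust for other valid hits.
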(event EventBeginPlay
  (bind _m_weaponabilitysystemcomponent (Variables|Default|Getm_WeaponAbilitySystemComponent))
  (Class|AbilitySystemComponent|InitStats _m_weaponabilitysystemcomponent "/Script/Outpost_Production.BaseWeaponAttributeSet" "/Game/Blueprints/Weapons/MainWeapons/Shotgun/ShotgunDataTable.ShotgunDataTable")
  (GameplayEffects|ApplyGameplayEffectToSelf :self _m_weaponabilitysystemcomponent :GameplayEffectClass "/Game/Blueprints/Weapons/MainWeapons/Shotgun/GE_Shotgun_Tags.GE_Shotgun_Tags_C"))

(event EventWeaponFireEvent
  (Animation|Montage|PlayMontage (Variables|Default|GetSkeletalMeshComponent) "/Game/Assets/3D_Assets/Character/Weapons/Shotgun/SK_Shotgun_Fire_Montage.SK_Shotgun_Fire_Montage"
    (:then
      (Audio|PlaySoundatLocation (Variables|Default|Getm_FireSoundEffect) (Transformation|GetActorLocation) "0, 0, 0" 1.0 1.0 0.0 0 0 0)
      (Components|Activation|Activate (Variables|Default|GetNS_MuzzleFlash) true)
      (Niagara|SetNiagaraVariable(Vector3) (Variables|Default|GetNS_MuzzleFlash) "User.Direction" (Math|Vector|GetRightVector (Variables|Default|GetSkeletalMeshComponent))))))

(event EventWeaponHitEvent
  (params (endLocation :type Vector :default "0, 0, 0") (hitActor :type Actor%20Object%20Reference))
  (bind _skeletalmeshcomponent (Variables|Default|GetSkeletalMeshComponent))
  (bind _returnvalue (Transformation|GetSocketLocation _skeletalmeshcomponent "Muzzle_Socket"))
  (bind _returnvalue_2 (- endLocation _returnvalue))
  (bind _returnvalue_3 (Math|Vector|Normalize _returnvalue_2))
  (bind _returnvalue_4 (Niagara|SpawnSystematLocation "/Game/Assets/VFX/ParticleSystems/BulletTrace/NS_BulletTrail.NS_BulletTrail" _returnvalue))
  (Niagara|SetNiagaraVariable(Vector3) _returnvalue_4 "User.DirectionVector" _returnvalue_3)
  (Niagara|SetNiagaraVariable(Vector3) _returnvalue_4 "User.FacingVector" _returnvalue_3)
  (Utilities|IsValid hitActor
    (:Is%20Valid
      (if (Actor|ActorHasTag hitActor "Enemy")
        (Niagara|SpawnSystematLocation "/Game/Assets/VFX/ParticleSystems/WeaponHitEffects/HitEnemy/NS_BloodSplatter.NS_BloodSplatter" endLocation "0, 0, 0" "1.000000,1.000000,1.000000" true true "AutoRelease")
        (else
          (Niagara|SpawnSystematLocation "/Game/Assets/VFX/ParticleSystems/WeaponHitEffects/DustHit/NS_DustHIt.NS_DustHIt" endLocation "0, 0, 0" "1.000000,1.000000,1.000000" true true "AutoRelease"))))))

(fn ConstructionScript)