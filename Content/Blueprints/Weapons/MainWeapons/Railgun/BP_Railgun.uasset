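; Railgun weapon Blueprint that handles the gun's charge, shot and hit feedback.
; On BeginPlay it initializes ability system stats from a data table, applies a tag effect and prints the first owned tag.
; Starting fire runs charge VFX and audio; stopping fire ends them, then plays the shot sound and fire montage.
; Hit events spawn an auto-released pooled Niagara flash at the end location.
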(event EventBeginPlay
  (bind _m_weaponabilitysystemcomponent (Variables|Default|Getm_WeaponAbilitySystemComponent))
  (Class|AbilitySystemComponent|InitStats (Variables|Default|Getm_WeaponAbilitySystemComponent) "/Script/Outpost_Production.BaseWeaponAttributeSet" "/Game/Blueprints/Weapons/MainWeapons/Railgun/RailgunDataTable.RailgunDataTable")
  (GameplayEffects|ApplyGameplayEffectToSelf :self _m_weaponabilitysystemcomponent :GameplayEffectClass "/Game/Blueprints/Weapons/MainWeapons/Railgun/GE_Railgun_Tags.GE_Railgun_Tags_C")
  (Development|PrintString (Utilities|String|ToString(Name) (GameplayTags|GetTagName (Utilities|Array|Get(acopy) (GameplayTags|BreakGameplayTagContainer (GameplayTags|GetOwnedGameplayTags _m_weaponabilitysystemcomponent :!class /Script/GameplayTags.GameplayTagAssetInterface)))))))

(event EventWeaponFireEvent
  (Components|Activation|Activate (Variables|Default|GetNS_Charge) true)
  (Audio|Components|Audio|Play (Variables|Default|Getm_AudioComponent) 0.0))

(event EventWeaponStopFireEvent
  (Components|Activation|Deactivate (Variables|Default|GetNS_Charge))
  (Audio|Components|Audio|Stop (Variables|Default|Getm_AudioComponent))
  (Audio|PlaySoundatLocation "/Game/Assets/Sound/FX/Weapons/RailgunShot_Cue.RailgunShot_Cue" (Transformation|GetActorLocation) "0, 0, 0" 1.0 1.0 0.0 "/Game/Blueprints/Audio/BP_EffectAttenuation.BP_EffectAttenuation" 0 0)
  (Animation|Montage|PlayMontage (Variables|Default|GetSkeletalMeshComponent) "/Game/Assets/3D_Assets/Character/Weapons/Railgun/SK_Railgun_Fire_Montage.SK_Railgun_Fire_Montage"))

(event EventWeaponHitEvent
  (params (endLocation :type Vector :default "0, 0, 0") (hitActor :type Actor%20Object%20Reference))
  (Niagara|SpawnSystematLocation "/Game/Assets/VFX/ParticleSystems/Railgun/Hit/NS_RailgunHitFlash.NS_RailgunHitFlash" endLocation "0, 0, 0" "1.000000,1.000000,1.000000" true true "AutoRelease"))

(fn ConstructionScript)