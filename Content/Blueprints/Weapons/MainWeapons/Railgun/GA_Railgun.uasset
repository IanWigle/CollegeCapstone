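; Railgun Gameplay Ability that fires a piercing multi-line trace for either a player mech or an AI turret, damaging every Enemy-tagged hit through GE_Damage with SetByCaller magnitude.
; The player path waits for input release, traces from the camera, scales damage by a clamped power curve of hold time, and multicasts weapon effects.
; The turret path waits an attribute-driven delay, then traces to its blackboard target for flat damage, toggling CanFire around the shot.
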(event Ability|EventActivateAbility
  (bind _returnvalue (Ability|GetOwningActorfromActorInfo))
  (bind _asbase_weapon (Utilities|Casting|CastToBaseWeapon (Ability|GetAvatarActorfromActorInfo)))
  (Variables|Default|SetWeapon _asbase_weapon)
  (bind _asbp_player_mech (Utilities|Casting|CastToBP_PlayerMech _returnvalue)
    (:then
      (Variables|Default|SetPlayer _asbp_player_mech)
      (bind _payload (Ability|Tasks|WaitGameplayEvent "(TagName=\"Weapon.InputReleased\")" 0)
        (:then
          (Class|BaseWeapon|NetMulticastWeaponFireStarted (Variables|Default|GetWeapon)))
        (:EventReceived
          (Variables|Default|SetTimeHeld (.EventMagnitude (Utilities|Struct|BreakGameplayEventData _payload)))
          (bind _outhits (Collision|MultiLineTraceByChannel (Transformation|GetWorldLocation (Variables|/Script/Outpost_Production.PlayerMech|Getm_FollowCamera (Variables|Default|GetPlayer))) (+ (Transformation|GetWorldLocation (Variables|/Script/Outpost_Production.PlayerMech|Getm_FollowCamera (Variables|Default|GetPlayer))) (* (Math|Vector|GetForwardVector (Variables|/Script/Outpost_Production.PlayerMech|Getm_FollowCamera (Variables|Default|GetPlayer))) (Math|Conversions|ToVector(Float) (.ReturnValue (Ability|Attribute|GetFloatAttribute (Variables|Default|GetWeapon) "(AttributeName=\"\",Attribute=StructProperty'\"/Script/Outpost_Production.BaseWeaponAttributeSet:m_HardRange\"',AttributeOwner=None)"))))) "TraceTypeQuery4" false (Utilities|Array|MakeArray (Variables|Default|GetWeapon) (Variables|Default|GetPlayer)) "ForDuration"))
          (for _array_element _outhits
            (Utilities|IsValid (.HitActor (Collision|BreakHitResult _array_element))
              (:Is%20Valid
                (Class|BaseWeapon|NetMulticastWeaponHit (Variables|Default|GetWeapon) (.Location (Collision|BreakHitResult _array_element)) (.HitActor (Collision|BreakHitResult _array_element)))
                (if (Actor|ActorHasTag (.HitActor (Collision|BreakHitResult _array_element)) "Enemy")
                  (bind _returnvalue_2 (Ability|GameplayEffect|AssignTagSetbyCallerMagnitude (Ability|MakeOutgoingGameplayEffectSpec "/Game/Blueprints/Weapons/GE_Damage.GE_Damage_C") "(TagName=\"Damage\")" (* (Math|Float|Clamp(Float) (Math|Float|Power (Variables|Default|GetTimeHeld) (/ (Math|Float|Loge (.ReturnValue (Ability|Attribute|GetFloatAttribute (Variables|Default|GetWeapon) "(AttributeName=\"\",Attribute=StructProperty'\"/Script/Outpost_Production.BaseWeaponAttributeSet:m_Damage\"',AttributeOwner=None)"))) (Math|Float|Loge (.ReturnValue (Ability|Attribute|GetFloatAttribute (Variables|Default|GetWeapon) "(AttributeName=\"\",Attribute=StructProperty'\"/Script/Outpost_Production.BaseWeaponAttributeSet:m_FireRate\"',AttributeOwner=None)"))))) 1.0 (.ReturnValue (Ability|Attribute|GetFloatAttribute (Variables|Default|GetWeapon) "(AttributeName=\"\",Attribute=StructProperty'\"/Script/Outpost_Production.BaseWeaponAttributeSet:m_Damage\"',AttributeOwner=None)"))) -1.0)))
                  (GameplayEffects|ApplyGameplayEffectSpecToTarget _returnvalue_2 (Ability|TargetData|AbilityTargetDatafromHitResult _array_element))))))
          (Class|BaseWeapon|NetMulticastWeaponStopFire (Variables|Default|GetWeapon))
          (Ability|EndAbility))))
    (:CastFailed
      (bind _asbp_turret (Utilities|Casting|CastToBP_Turret _returnvalue)
        (:then
          (bind _output_get (Variables|Default|SetTurret _asbp_turret))
          (Utilities|IsValid (Variables|/Script/Outpost_Production.Turret|Getm_CurrentTarget _output_get)
            (:Is%20Valid
              (bind _asaicontroller (Utilities|Casting|CastToAIController (Pawn|GetController (Variables|Default|GetTurret)))
                (:then
                  (if (ScalableFloat|GetValueasBool (AI|GetBlackboard _asaicontroller) (Utilities|Name|MakeLiteralName "CanFire"))
                    (bind _output_get_2 (Variables|Default|SetWeapon (Variables|/Script/Outpost_Production.Turret|Getm_ActiveTurretWeapon (Variables|Default|GetTurret))))
                    (Ability|Tasks|WaitDelay (.ReturnValue (Ability|Attribute|GetFloatAttribute _output_get_2 "(AttributeName=\"m_FireRate\",Attribute=StructProperty'\"/Script/Outpost_Production.BaseWeaponAttributeSet:m_FireRate\"',AttributeOwner=Class'\"/Script/Outpost_Production.BaseWeaponAttributeSet\"')"))
                      (:then
                        (bind _asaicontroller_2 (Utilities|Casting|CastToAIController (Pawn|GetController (Variables|Default|GetTurret)))
                          (:then
                            (AI|Components|Blackboard|SetValueasBool (AI|GetBlackboard _asaicontroller_2) (Utilities|Name|MakeLiteralName "CanFire") false))
                          (:CastFailed
                            (Ability|EndAbility))))
                      (:OnFinish
                        (Utilities|IsValid (Variables|/Script/Outpost_Production.Turret|Getm_CurrentTarget (Variables|Default|GetTurret))
                          (:Is%20Valid
                            (bind _asactor (Utilities|Casting|CastToActor (AI|Components|Blackboard|GetValueasObject (AI|GetBlackboard (Variables|Default|GetTurret)) (Utilities|Name|MakeLiteralName "CurrentTarget")))
                              (:then
                                (bind _outhits_2 (Collision|MultiLineTraceByChannel (Transformation|GetActorLocation (Variables|Default|GetWeapon)) (Transformation|GetActorLocation _asactor) "TraceTypeQuery4" false (Utilities|Array|MakeArray (Variables|Default|GetWeapon) (Variables|Default|GetTurret) 0) "ForDuration"))
                                (for _array_element_2 _outhits_2
                                  (Utilities|IsValid (.HitActor (Collision|BreakHitResult _array_element_2))
                                    (:Is%20Valid
                                      (if (Actor|ActorHasTag (.HitActor (Collision|BreakHitResult _array_element_2)) "Enemy")
                                        (bind _returnvalue_3 (Ability|GameplayEffect|AssignTagSetbyCallerMagnitude (Ability|MakeOutgoingGameplayEffectSpec "/Game/Blueprints/Weapons/GE_Damage.GE_Damage_C") "(TagName=\"Damage\")" (* (.ReturnValue (Ability|Attribute|GetFloatAttribute (Variables|Default|GetWeapon) "(AttributeName=\"m_Damage\",Attribute=StructProperty'\"/Script/Outpost_Production.BaseWeaponAttributeSet:m_Damage\"',AttributeOwner=Class'\"/Script/Outpost_Production.BaseWeaponAttributeSet\"')")) -1.0)))
                                        (GameplayEffects|ApplyGameplayEffectSpecToTarget _returnvalue_3 (Ability|TargetData|AbilityTargetDatafromHitResult _array_element_2))))))
                                (bind _asaicontroller_3 (Utilities|Casting|CastToAIController (Pawn|GetController (Variables|Default|GetTurret)))
                                  (:then
                                    (AI|Components|Blackboard|SetValueasBool (AI|GetBlackboard _asaicontroller_3) (Utilities|Name|MakeLiteralName "CanFire") true)
                                    (Ability|EndAbility))
                                  (:CastFailed
                                    (Ability|EndAbility))))
                              (:CastFailed
                                (Ability|EndAbility))))
                          (:Is%20Not%20Valid
                            (Ability|EndAbility)))))
                    (else
                      (Ability|EndAbility :!label _label))))
                (:CastFailed
                  (goto _label))))
            (:Is%20Not%20Valid
              (Ability|EndAbility))))
        (:CastFailed
          (Ability|EndAbility))))))

(fn CreateDamageSpec)