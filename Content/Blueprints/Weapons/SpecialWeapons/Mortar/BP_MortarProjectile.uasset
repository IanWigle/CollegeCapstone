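; Mortar projectile for a special weapon that explodes on actor overlap or mesh hit and then destroys itself.
; The explosion spawns a Niagara effect and sound at the mesh location, then runs a debug-drawn multi-sphere trace around that point.
; Hit actors tagged Enemy are cast to BaseEnemy and receive damage through a stored Gameplay Ability System effect spec.
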(event OnComponentHit(StaticMesh)
  (params (HitComponent :type Primitive%20Component%20Object%20Reference) (OtherActor :type Actor%20Object%20Reference) (OtherComp :type Primitive%20Component%20Object%20Reference) (NormalImpulse :type Vector :default "0, 0, 0") (Hit :type Hit%20Result%20Structure%20%28by%20ref%29))
  (bind _staticmesh (Variables|Default|GetStaticMesh))
  (bind _returnvalue (Transformation|GetWorldLocation _staticmesh))
  (Niagara|SpawnSystematLocation "/Game/Assets/VFX/ParticleSystems/MortarExplosion/NS_MortarExplosion.NS_MortarExplosion" _returnvalue)
  (Audio|PlaySoundatLocation "/Game/Assets/Sound/FX/Weapons/explosion_Cue.explosion_Cue" _returnvalue "0, 0, 0" 1.0 1.0 0.0 0 0 0)
  (bind _outhits (Collision|MultiSphereTraceByChannel _returnvalue _returnvalue 1e+03 "TraceTypeQuery3" false 0 "ForDuration"))
  (for _array_element _outhits
    (Utilities|IsValid (.HitActor (Collision|BreakHitResult _array_element))
      (:Is%20Valid
        (if (Actor|ActorHasTag (.HitActor (Collision|BreakHitResult _array_element)) "Enemy")
          (bind _asbase_enemy (Utilities|Casting|CastToBaseEnemy (.HitActor (Collision|BreakHitResult _array_element))))
          (GameplayEffects|ApplyGameplayEffectSpecToSelf (Ability|GetAbilitySystemComponent _asbase_enemy) (Variables|Default|GetDamageEffectSpecHandle))))))
  (Actor|DestroyActor))

(event Collision|EventActorBeginOverlap
  (params (OtherActor :type Actor%20Object%20Reference))
  (bind _staticmesh (Variables|Default|GetStaticMesh))
  (bind _returnvalue (Transformation|GetWorldLocation _staticmesh))
  (Niagara|SpawnSystematLocation "/Game/Assets/VFX/ParticleSystems/MortarExplosion/NS_MortarExplosion.NS_MortarExplosion" _returnvalue)
  (Audio|PlaySoundatLocation "/Game/Assets/Sound/FX/Weapons/explosion_Cue.explosion_Cue" _returnvalue "0, 0, 0" 1.0 1.0 0.0 0 0 0)
  (bind _outhits (Collision|MultiSphereTraceByChannel _returnvalue _returnvalue 1e+03 "TraceTypeQuery3" false 0 "ForDuration"))
  (for _array_element _outhits
    (Utilities|IsValid (.HitActor (Collision|BreakHitResult _array_element))
      (:Is%20Valid
        (if (Actor|ActorHasTag (.HitActor (Collision|BreakHitResult _array_element)) "Enemy")
          (bind _asbase_enemy (Utilities|Casting|CastToBaseEnemy (.HitActor (Collision|BreakHitResult _array_element))))
          (GameplayEffects|ApplyGameplayEffectSpecToSelf (Ability|GetAbilitySystemComponent _asbase_enemy) (Variables|Default|GetDamageEffectSpecHandle))))))
  (Actor|DestroyActor))

(fn ConstructionScript)