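; Gameplay ability for a mech's mortar special weapon, with hold-to-aim and release-to-fire input.
; Unless the weapon is reloading, it raises the follow camera and runs a BP_MortarTarget targeting task, confirmed by the input-released event.
; On commit it multicasts fire start; the authority then launches a projectile along a suggested arc, carrying SetByCaller damage.
; The authority also lowers the camera and applies a timed reload effect to the weapon.
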(event Ability|EventActivateAbility
  (bind _returnvalue (Class|GameplayAbility|MakeTargetLocationInfofromOwnerActor))
  (bind (_locationtype _literaltransform _sourceactor _sourcecomponent _sourceability _sourcesocketname) (Utilities|Struct|BreakGameplayAbilityTargetingLocationInfo _returnvalue))
  ;[1 1 1] Setting the player character
  (bind _asbase_weapon (Utilities|Casting|CastToBaseWeapon (Ability|GetAvatarActorfromActorInfo)))
  (Variables|Default|SetOwningWeapon _asbase_weapon)
  (bind _asplayer_mech (Utilities|Casting|CastToPlayerMech (Ability|GetOwningActorfromActorInfo))
    (:then
      (Variables|Default|SetOwning%20Player%20Character _asplayer_mech)
      (if (GameplayTags|HasAnyMatchingGameplayTags (Ability|GetAbilitySystemComponent (Variables|Default|GetOwningWeapon)) (GameplayTags|MakeGameplayTagContainerfromArray (Utilities|Array|MakeArray (GameplayTags|MakeLiteralGameplayTag "(TagName=\"Weapon.Reloading\")"))))
        (Ability|EndAbility)
        (else
          (Transformation|SetWorldLocation (Variables|/Script/Outpost_Production.PlayerMech|Getm_FollowCamera (Variables|Default|GetOwning%20Player%20Character)) (+ (Transformation|GetWorldLocation (Variables|/Script/Outpost_Production.PlayerMech|Getm_FollowCamera (Variables|Default|GetOwning%20Player%20Character))) (Math|Vector|MakeVector 0.0 0.0 (Variables|Default|GetCameraOffset))) false true)
          (bind (_asynctaskproxy _data) (|WaitTargetData :TaskInstanceName "Targeting" :ConfirmationType "Custom" :Class "/Game/Blueprints/Weapons/SpecialWeapons/Mortar/BP_MortarTarget.BP_MortarTarget_C" :TraceProfile "(Name=\"TaergetActorGroundLocation\")" :StartLocation (Utilities|Struct|MakeGameplayAbilityTargetingLocationInfo _locationtype (Math|Transform|MakeTransform (+ (* (Transformation|GetActorForwardVector (Variables|Default|GetOwning%20Player%20Character)) 2e+02) (.location _literaltransform)) (.rotation _literaltransform) (.scale _literaltransform)) _sourceactor _sourcecomponent _sourceability _sourcesocketname) :ReticleClass 0)
            (:then
              (Variables|Default|SetTargetingTask _asynctaskproxy)
              (Ability|Tasks|WaitGameplayEvent "(TagName=\"Weapon.InputReleased\")" 0
                (:EventReceived
                  (Class|GameplayAbility|ConfirmTaskbyInstanceName "Targeting" false))))
            (:ValidData
              (bind _returnvalue_2 (Ability|CommitAbility))
              (if _returnvalue_2
                (Class|BaseWeapon|NetMulticastWeaponFireStarted (Variables|Default|GetOwningWeapon))
                (if (Ability|HasAuthority (Variables|Default|GetOwning%20Player%20Character))
                  (bind _returnvalue_3 (Game|SpawnActorfromClass "/Game/Blueprints/Weapons/SpecialWeapons/Mortar/BP_MortarProjectile.BP_MortarProjectile_C" (Math|Transform|MakeTransform (Transformation|GetSocketLocation (Variables|/Script/Engine.SkeletalMeshActor|GetSkeletalMeshComponent (Variables|Default|GetOwningWeapon)) "Socket_Muzzle") "0, 0, 0" "1,1,1") "AlwaysSpawn" 0 0))
                  (bind _returnvalue_4 (Ability|GameplayEffect|AssignTagSetbyCallerMagnitude (Ability|MakeOutgoingGameplayEffectSpec "/Game/Blueprints/Weapons/GE_Damage.GE_Damage_C") "(TagName=\"Damage\")" (* -1 (.ReturnValue (Ability|Attribute|GetFloatAttribute (Variables|Default|GetOwningWeapon) "(AttributeName=\"m_Damage\",Attribute=StructProperty'\"/Script/Outpost_Production.BaseWeaponAttributeSet:m_Damage\"',AttributeOwner=Class'\"/Script/Outpost_Production.BaseWeaponAttributeSet\"')")))))
                  (Variables|/Game/Blueprints/Weapons/SpecialWeapons/Mortar/BP_MortarProjectile.BP_MortarProjectile_C|SetDamageEffectSpecHandle _returnvalue_3 _returnvalue_4)
                  (bind _outlaunchvelocity (Game|SuggestProjectileVelocityCustomArc (Transformation|GetSocketLocation (Variables|/Script/Engine.SkeletalMeshActor|GetSkeletalMeshComponent (Variables|Default|GetOwningWeapon)) "Socket_Muzzle") (.Location (Collision|BreakHitResult (Ability|TargetData|GetHitResultfromTargetData _data))) 0.0 0.5))
                  (Physics|AddImpulse (Variables|/Game/Blueprints/Weapons/SpecialWeapons/Mortar/BP_MortarProjectile.BP_MortarProjectile_C|GetStaticMesh _returnvalue_3) _outlaunchvelocity "None" true)
                  (Transformation|SetWorldLocation (Variables|/Script/Outpost_Production.PlayerMech|Getm_FollowCamera (Variables|Default|GetOwning%20Player%20Character)) (+ (Transformation|GetWorldLocation (Variables|/Script/Outpost_Production.PlayerMech|Getm_FollowCamera (Variables|Default|GetOwning%20Player%20Character))) (Math|Vector|MakeVector 0.0 0.0 (* -1 (Variables|Default|GetCameraOffset)))) false true)
                  (bind _returnvalue_5 (Ability|GameplayEffect|AssignTagSetbyCallerMagnitude (Ability|MakeOutgoingGameplayEffectSpec "/Game/Blueprints/Weapons/MainWeapons/GE_Reload.GE_Reload_C") "(TagName=\"Weapon.Reloading\")" (.ReturnValue (Ability|Attribute|GetFloatAttribute (Variables|Default|GetOwningWeapon) "(AttributeName=\"\",Attribute=StructProperty'\"/Script/Outpost_Production.BaseWeaponAttributeSet:m_ReloadSpeed\"',AttributeOwner=None)"))))
                  (GameplayEffects|ApplyGameplayEffectSpecToTarget _returnvalue_5 (Ability|TargetData|AbilityTargetDatafromActor (Variables|Default|GetOwningWeapon)))
                  (Ability|EndAbility)
                  (else
                    (Ability|EndAbility)))
                (else
                  (Ability|CancelAbility :!label _label))))
            (:Cancelled
              (goto _label))))))
    (:CastFailed
      (Development|PrintString "GA_Mortar - Cast to Player Mech Failed")
      (Ability|EndAbility))))