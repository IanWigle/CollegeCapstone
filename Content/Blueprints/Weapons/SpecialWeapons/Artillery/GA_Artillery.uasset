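; GA_Artillery is the gameplay ability for the mech's artillery special weapon, firing a homing projectile at whatever the player aims at.
; Activation raises the follow camera until input release, then line-traces along its view and spawns BP_ArtilleryProjectile at the muzzle, homing on the hit component.
; The camera is then restored, and the ability waits for a gameplay event before ending.
; ResetCamera restores the camera arm but is not called here.
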(event Ability|EventActivateAbility
  (bind _asbase_weapon (Utilities|Casting|CastToBaseWeapon (Ability|GetCurrentSourceObject))
    (:then
      (bind _output_get (Variables|Default|SetWeapon _asbase_weapon))
      (bind _asplayer_mech (Utilities|Casting|CastToPlayerMech (Components|GetOwner _output_get))
        (:then
          (bind _output_get_2 (Variables|Default|SetPlayer _asplayer_mech))
          (bind _output_get_3 (Variables|Default|SetPlayerCamera (Variables|/Script/Outpost_Production.PlayerMech|Getm_FollowCamera _output_get_2)))
          (bind _output_get_4 (Variables|Default|SetOriginalLocation (Variables|/Script/Engine.SceneComponent|GetRelativeLocation _output_get_3)))
          (Transformation|SetRelativeLocation _output_get_3 (+ _output_get_4 "0,0.000000,1000.000000") false false)
          (Ability|Tasks|WaitInputRelease false
            (:OnRelease
              (bind _outhit (Class|KismetSystemLibrary|LineTraceSinglebyProfile (Transformation|GetWorldLocation (Variables|Default|GetPlayerCamera)) (+ (Transformation|GetWorldLocation (Variables|Default|GetPlayerCamera)) (* (Math|Vector|GetForwardVector (Variables|Default|GetPlayerCamera)) 1e+05)) "BlockAll" false 0 "ForDuration" true))
              (bind _returnvalue (Game|SpawnActorfromClass "/Game/Blueprints/Weapons/SpecialWeapons/Artillery/BP_ArtilleryProjectile.BP_ArtilleryProjectile_C" (Math|Transform|MakeTransform (Transformation|GetSocketLocation (Variables|/Script/Engine.SkeletalMeshActor|GetSkeletalMeshComponent (Variables|Default|GetWeapon)) "Muzzle_Socket") "0, 0, 0" "1,1,1") "AlwaysSpawn" (Variables|Default|GetPlayer) (Variables|Default|GetPlayer)))
              (Variables|/Script/Engine.ProjectileMovementComponent|SetHomingTargetComponent (Variables|/Script/Outpost_Production.Projectile|Getm_ProjectileComponent _returnvalue) (.HitComponent (Collision|BreakHitResult _outhit)))
              (Transformation|SetRelativeLocation (Variables|Default|GetPlayerCamera) (Variables|Default|GetOriginalLocation) false false)
              (Ability|Tasks|WaitGameplayEvent :OptionalExternalTarget 0
                (:EventReceived
                  (Ability|EndAbility))))))
        (:CastFailed
          (Development|PrintString "GAAtrillery: Failed to cast owner to playermech"))))
    (:CastFailed
      (Development|PrintString "GAArtillery: Failed to cast to base weapon!"))))

(fn ResetCamera
  (bind _player (Variables|Default|GetPlayer))
  (Transformation|SetRelativeLocation (Variables|/Script/Outpost_Production.PlayerMech|Getm_CameraArm _player) (Variables|/Script/Outpost_Production.PlayerMech|Getm_CameraArmStartingLocation _player) false false))