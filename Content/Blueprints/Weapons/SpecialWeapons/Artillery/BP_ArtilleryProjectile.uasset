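; Projectile for the Artillery special weapon that reports its impact and removal back to the owning PlayerMech through gameplay events.
; On hit it spawns a pooled explosion effect, sends a Hit event carrying the struck actor as Instigator and the impact location as target data, then destroys itself.
; Any destruction sends a Despawned event to the owner; the projectile applies no damage in these graphs.
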(event EventDestroyed
  (bind _asplayer_mech (Utilities|Casting|CastToPlayerMech (Components|GetOwner)))
  (Ability|SendGameplayEventtoActor _asplayer_mech "(TagName=\"Weapon.Special.Artillery.Despawned\")"))

(event Collision|EventHit
  (params (MyComp :type Primitive%20Component%20Object%20Reference) (Other :type Actor%20Object%20Reference) (OtherComp :type Primitive%20Component%20Object%20Reference) (bSelfMoved :type Boolean) (HitLocation :type Vector :default "0, 0, 0") (HitNormal :type Vector :default "0, 0, 0") (NormalImpulse :type Vector :default "0, 0, 0") (Hit :type Hit%20Result%20Structure%20%28by%20ref%29))
  (bind _returnvalue (Math|Conversions|ToTransform(Vector) HitLocation))
  (bind _gameplayabilitytargetinglocationinfo (Utilities|Struct|MakeGameplayAbilityTargetingLocationInfo "LiteralTransform" _returnvalue))
  (Effects|SpawnEmitteratLocation "/Game/StarterContent/Particles/P_Explosion.P_Explosion" HitLocation "0, 0, 0" "1.000000,1.000000,1.000000" true "AutoRelease")
  (bind _asplayer_mech (Utilities|Casting|CastToPlayerMech (Components|GetOwner)))
  (Ability|SendGameplayEventtoActor _asplayer_mech "(TagName=\"Weapon.Special.Artillery.Hit\")" (Utilities|Struct|MakeGameplayEventData "" Other 0 0 0 "()" "(GameplayTags=)" "(GameplayTags=)" 0.0 (Class|AbilitySystemBlueprintLibrary|AbilityTargetDatafromLocations _gameplayabilitytargetinglocationinfo _gameplayabilitytargetinglocationinfo)))
  (Actor|DestroyActor))

(fn ConstructionScript)