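; Gameplay ability for the HSM special weapon that fires a salvo of homing rockets from the player mech.
; Unless the weapon is reloading, it stops the mech and halves its walk speed during a timed delay, then box-traces from the camera using viewport-derived extents.
; Pooled projectiles launch from weapon sockets, spread round-robin across living enemies found.
; It then restores speed, applies GE_Reload to the weapon and ends.
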(event Ability|EventActivateAbility
  (bind _returnvalue (Viewport|GetViewportSize))
  (bind _enemies (Variables|Objects|GetEnemies))
  (bind (_x _y) (Math|Vector2D|BreakVector2D _returnvalue))
  (bind _asbp_hsm (Utilities|Casting|CastToBP_HSM (Ability|GetAvatarActorfromActorInfo))
    (:then
      (bind _output_get (Variables|Objects|SetWeapon _asbp_hsm))
      (if (GameplayTags|HasAnyMatchingGameplayTags (Ability|GetAbilitySystemComponent (Variables|Objects|GetWeapon)) (GameplayTags|MakeGameplayTagContainerfromArray (Utilities|Array|MakeArray (GameplayTags|MakeLiteralGameplayTag "(TagName=\"Weapon.Reloading\")"))))
        (Ability|EndAbility)
        (else
          (Variables|TargetData|SetNumberOfRocketsToSpawn (Variables|/Script/Outpost_Production.ProjectileWeapon|Getm_NumProjectiles _output_get))
          (bind _asplayer_mech (Utilities|Casting|CastToPlayerMech (Ability|GetOwningActorfromActorInfo))
            (:then
              (Variables|Objects|SetPlayer _asplayer_mech)
              (Ability|Tasks|WaitGameplayEvent "(TagName=\"Weapon.InputReleased\")" 0
                (:then
                  (Ability|Tasks|WaitDelay 3.0
                    (:then
                      ;[1 1 1] Stop Moving
                      (Components|Movement|StopMovementImmediately (Variables|/Script/Engine.Character|GetCharacterMovement (Variables|Objects|GetPlayer)))
                      ;[1 1 1] Reduce Movement by Half
                      (Variables|/Script/Engine.CharacterMovementComponent|SetMaxWalkSpeed (Variables|/Script/Engine.Character|GetCharacterMovement (Variables|Objects|GetPlayer)) (/ (Variables|/Script/Engine.CharacterMovementComponent|GetMaxWalkSpeed (Variables|/Script/Engine.Character|GetCharacterMovement (Variables|Objects|GetPlayer))) 2.0))
                      (Class|BaseWeapon|NetMulticastWeaponFireStarted (Variables|Objects|GetWeapon)))
                    (:OnFinish
                      (bind (_outhits _returnvalue_2) (Class|KismetSystemLibrary|BoxTraceMulti (Transformation|GetWorldLocation (Variables|/Script/Outpost_Production.PlayerMech|Getm_FollowCamera (Variables|Objects|GetPlayer))) (+ (Transformation|GetWorldLocation (Variables|/Script/Outpost_Production.PlayerMech|Getm_FollowCamera (Variables|Objects|GetPlayer))) (* (Math|Vector|GetForwardVector (Variables|/Script/Outpost_Production.PlayerMech|Getm_FollowCamera (Variables|Objects|GetPlayer))) (Variables|Default|GetMaxScanDistance))) (Math|Vector|MakeVector (* _x _y) (/ _x 2.0) (/ _y 2.0)) (Math|Conversions|RotationFromXVector (Math|Vector|GetForwardVector (Variables|/Script/Outpost_Production.PlayerMech|Getm_FollowCamera (Variables|Objects|GetPlayer)))) "TraceTypeQuery3" false (Utilities|Array|MakeArray (Variables|Objects|GetWeapon) (Variables|Objects|GetPlayer)) "ForDuration" true))
                      (if _returnvalue_2
                        ;[1 1 1] Check if the found enemies are valid to attack
                        (for _array_element _outhits
                          (bind _asbase_enemy (Utilities|Casting|CastToBaseEnemy (.HitActor (Collision|BreakHitResult _array_element))))
                          (if (not (Variables|/Script/Outpost_Production.BaseEntity|Getm_bIsDead _asbase_enemy))
                            (Utilities|Array|Add (Variables|Objects|GetEnemies) _asbase_enemy)))
                        (if (> (Utilities|Array|Length (Variables|Objects|GetEnemies)) 0)
                          (for _index (range 0 (- (Variables|TargetData|GetNumberOfRocketsToSpawn) 1))
                            (Variables|Objects|SetCurrentEnemy (Utilities|Array|Get(acopy) _enemies (Math|Integer|%(Integer) _index (Utilities|Array|Length _enemies))))
                            (bind _returnvalue_3 (Class|ProjectileWeapon|GetAvailableProjectile (Variables|Objects|GetWeapon)))
                            (Utilities|IsValid _returnvalue_3
                              (:Is%20Valid
                                (Class|Projectile|NetMulticastEnable _returnvalue_3 (.Location (Math|Transform|BreakTransform (Transformation|GetSocketTransform (Variables|/Script/Engine.SkeletalMeshActor|GetSkeletalMeshComponent (Variables|Objects|GetWeapon)) (Utilities|Array|Get(acopy) (Transformation|GetAllSocketNames (Variables|/Script/Engine.SkeletalMeshActor|GetSkeletalMeshComponent (Variables|Objects|GetWeapon))) _index) "RTS_World"))))
                                (Class|Projectile|AssignNewTarget _returnvalue_3 (Variables|Objects|GetCurrentEnemy))
                                (Class|Projectile|BeginLifeSpan _returnvalue_3))))))
                      ;[1 1 1] Reset Mech Movement
                      (Variables|/Script/Engine.CharacterMovementComponent|SetMaxWalkSpeed (Variables|/Script/Engine.Character|GetCharacterMovement (Variables|Objects|GetPlayer)) (* (Variables|/Script/Engine.CharacterMovementComponent|GetMaxWalkSpeed (Variables|/Script/Engine.Character|GetCharacterMovement (Variables|Objects|GetPlayer))) 2.0))
                      (Class|BaseWeapon|NetMulticastWeaponStopFire (Variables|Objects|GetWeapon))
                      (Ability|Tasks|WaitDelay 3.0
                        (:then
                          (bind _returnvalue_4 (Ability|GameplayEffect|AssignTagSetbyCallerMagnitude (Ability|MakeOutgoingGameplayEffectSpec "/Game/Blueprints/Weapons/MainWeapons/GE_Reload.GE_Reload_C") "(TagName=\"Weapon.Reloading\")" (.ReturnValue (Ability|Attribute|GetFloatAttribute (Variables|Objects|GetWeapon) "(AttributeName=\"\",Attribute=StructProperty'\"/Script/Outpost_Production.BaseWeaponAttributeSet:m_ReloadSpeed\"',AttributeOwner=None)"))))
                          (GameplayEffects|ApplyGameplayEffectSpecToTarget _returnvalue_4 (Ability|TargetData|AbilityTargetDatafromActor (Variables|Objects|GetWeapon)))
                          (Ability|EndAbility))
                        (:OnFinish
                          (Ability|EndAbility))))))))
            (:CastFailed
              (Ability|EndAbility))))))
    (:CastFailed
      (Ability|EndAbility))))

(event Ability|EventOnEndAbility
  (params (bWasCancelled :type Boolean))
  (Utilities|Array|Clear (Variables|Objects|GetEnemies)))

(fn EnableMissile
  (params (missile :type Projectile%20Object%20Reference) (new%20transform :type Transform))
  (Rendering|SetActorHiddenInGame missile false)
  (Actor|Tick|SetActorTickEnabled missile true)
  (Transformation|SetActorTransform missile new%20transform))

(fn AssignNewTarget
  (params (new%20Enemy :type Actor%20Object%20Reference) (missile :type Projectile%20Object%20Reference))
  (bind _m_projectilecomponent (Variables|/Script/Outpost_Production.Projectile|Getm_ProjectileComponent missile))
  (bind _output_get (Variables|/Script/Outpost_Production.Projectile|Setm_Target missile new%20Enemy))
  (Variables|/Script/Engine.ProjectileMovementComponent|SetHomingTargetComponent _m_projectilecomponent (Variables|/Script/Engine.Actor|GetRootComponent _output_get))
  (Variables|/Script/Engine.ProjectileMovementComponent|SetbIsHomingProjectile _m_projectilecomponent true)
  (Components|Activation|SetActive _m_projectilecomponent true false))