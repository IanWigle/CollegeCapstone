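; BP_HSM is the HSM special weapon Blueprint for a player mech, handling its ability setup and missile targeting HUD.
; On BeginPlay it initializes the weapon's ability system attributes from a data table and applies the HSM tags gameplay effect to itself.
; For locally controlled mechs only, firing creates or reuses the missile HUD widget and plays its startup animation, while stopping reverses that animation and plays audio.
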(event EventBeginPlay
  (bind _m_weaponabilitysystemcomponent (Variables|Default|Getm_WeaponAbilitySystemComponent))
  (Class|AbilitySystemComponent|InitStats _m_weaponabilitysystemcomponent "/Script/Outpost_Production.BaseWeaponAttributeSet" "/Game/Blueprints/Weapons/SpecialWeapons/HSM/HSMCannonDataTable.HSMCannonDataTable")
  (GameplayEffects|ApplyGameplayEffectToSelf :self _m_weaponabilitysystemcomponent :GameplayEffectClass "/Game/Blueprints/Weapons/SpecialWeapons/HSM/GE_HSM_Tags.GE_HSM_Tags_C"))

(event EventWeaponFireEvent
  (bind _asplayer_mech (Utilities|Casting|CastToPlayerMech (Components|GetOwner)))
  (if (Pawn|IsLocallyControlled _asplayer_mech)
    ;[1 1 1] Spawn and Add the Missile HUD Widget
    (bind _asplayer_controller (Utilities|Casting|CastToPlayerController (Pawn|GetController _asplayer_mech)))
    (Utilities|IsValid (Variables|Default|GetTargetWidget)
      (:Is%20Valid
        _)
      (:Is%20Not%20Valid
        (bind _returnvalue (UserInterface|CreateWidget "/Game/Blueprints/Weapons/SpecialWeapons/HSM/BP_MissileHUD.BP_MissileHUD_C" _asplayer_controller))
        (Variables|Default|SetTargetWidget _returnvalue)))
    (UserInterface|Animation|PlayAnimation (Variables|Default|GetTargetWidget) (Variables|/Game/Blueprints/Weapons/SpecialWeapons/HSM/BP_MissileHUD.BP_MissileHUD_C|GetStartup (Variables|Default|GetTargetWidget)) 0.0 1 "Forward" 1.0 false)
    (UserInterface|Viewport|AddtoViewport (Variables|Default|GetTargetWidget) 0)))

(event EventWeaponStopFireEvent
  (bind _targetwidget (Variables|Default|GetTargetWidget))
  (bind _asplayer_mech (Utilities|Casting|CastToPlayerMech (Components|GetOwner)))
  (if (Pawn|IsLocallyControlled _asplayer_mech)
    (Class|UserWidget|PlayAnimationReverse _targetwidget (Variables|/Game/Blueprints/Weapons/SpecialWeapons/HSM/BP_MissileHUD.BP_MissileHUD_C|GetStartup _targetwidget) 2.0 false)
    (Audio|Components|Audio|Play (Variables|Default|Getm_AudioComponent) 0.0)))

(fn ConstructionScript)