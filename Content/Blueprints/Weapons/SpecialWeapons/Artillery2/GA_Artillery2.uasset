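; GA_Artillery2 is the gameplay ability that fires a mech's artillery special weapon unless it is reloading.
; It spawns a projectile from the muzzle along controller rotation, using a replicated class on authority and a non-replicated one otherwise.
; A hit event triggers a sphere trace that applies area damage to Enemy-tagged actors and, if anything was traced, a SetByCaller reload effect.
; A despawn event ends the ability without reloading.
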(event Ability|EventActivateAbility
  ;[1 1 1] Setting the player character
  (bind _asbase_weapon (Utilities|Casting|CastToBaseWeapon (Ability|GetAvatarActorfromActorInfo)))
  (bind _output_get (Variables|Default|SetOwningWeapon _asbase_weapon))
  (bind _asplayer_mech (Utilities|Casting|CastToPlayerMech (Components|GetOwner _output_get))
    (:then
      (Variables|Default|SetOwning%20Player%20Character _asplayer_mech)
      (if (not (GameplayTags|HasAnyMatchingGameplayTags (Ability|GetAbilitySystemComponent (Variables|Default|GetOwningWeapon)) (GameplayTags|MakeGameplayTagContainerfromArray (Utilities|Array|MakeArray (GameplayTags|MakeLiteralGameplayTag "(TagName=\"Weapon.Reloading\")")))))
        (Ability|CommitAbility)
        (bind _asbase_weapon_2 (Utilities|Casting|CastToBaseWeapon (Ability|GetCurrentSourceObject)))
        (Game|SpawnActorfromClass (select (Utilities|Enum|Equal(Enum) (Utilities|Struct|BreakGameplayAbilityActivationInfo (Variables|Default|GetCurrentActivationInfo)) "Authority") "/Game/Blueprints/Weapons/SpecialWeapons/Artillery2/ArtilleryReplicatedProjectile.ArtilleryReplicatedProjectile_C" "/Game/Blueprints/Weapons/SpecialWeapons/Artillery2/ArtilleryNonReplicatedProjectile.ArtilleryNonReplicatedProjectile_C") (Math|Transform|MakeTransform (+ (Math|Vector|MakeVector 0.0 0.0 5e+01) (Transformation|GetSocketLocation (Variables|/Script/Engine.SkeletalMeshActor|GetSkeletalMeshComponent _asbase_weapon_2) "Muzzle_Socket")) (Transformation|GetActorRotation (Pawn|GetController (Variables|Default|GetOwning%20Player%20Character))) "1,1,1") "AlwaysSpawn" (Variables|Default|GetOwningWeapon) (Variables|Default|GetOwning%20Player%20Character))
        (bind _payload (Ability|Tasks|WaitGameplayEvent "(TagName=\"Weapon.Special.Artillery.Hit\")" 0)
          (:then
            (Ability|Tasks|WaitGameplayEvent "(TagName=\"Weapon.Special.Artillery.Despawned\")" 0
              (:EventReceived
                (Ability|EndAbility))))
          (:EventReceived
            (bind (_outhits _returnvalue) (Collision|MultiSphereTraceByChannel (.Location (Math|Transform|BreakTransform (Class|AbilitySystemBlueprintLibrary|GetTargetDataOrigin (.TargetData (Utilities|Struct|BreakGameplayEventData _payload))))) (.Location (Math|Transform|BreakTransform (Class|AbilitySystemBlueprintLibrary|GetTargetDataOrigin (.TargetData (Utilities|Struct|BreakGameplayEventData _payload))))) 2e+03 "TraceTypeQuery3" false 0 "ForDuration"))
            (if _returnvalue
              (for _array_element _outhits
                (Utilities|IsValid (.HitActor (Collision|BreakHitResult _array_element))
                  (:Is%20Valid
                    (if (Actor|ActorHasTag (.HitActor (Collision|BreakHitResult _array_element)) "Enemy")
                      (GameplayEffects|ApplyGameplayEffectToTarget :self (Ability|GetAbilitySystemComponent (Variables|Default|GetOwningWeapon)) :GameplayEffectClass "/Game/Blueprints/Weapons/SpecialWeapons/Artillery2/ArtilleryAOEDamage.ArtilleryAOEDamage_C" :Target (Ability|GetAbilitySystemComponent (.HitActor (Collision|BreakHitResult _array_element))))))))
              (bind _returnvalue_2 (Ability|GameplayEffect|AssignTagSetbyCallerMagnitude (Ability|MakeOutgoingGameplayEffectSpec "/Game/Blueprints/Weapons/MainWeapons/GE_Reload.GE_Reload_C") "(TagName=\"Weapon.Reloading\")" (.ReturnValue (Ability|Attribute|GetFloatAttribute (Variables|Default|GetOwningWeapon) "(AttributeName=\"\",Attribute=StructProperty'\"/Script/Outpost_Production.BaseWeaponAttributeSet:m_ReloadSpeed\"',AttributeOwner=None)"))))
              (GameplayEffects|ApplyGameplayEffectSpecToTarget _returnvalue_2 (Ability|TargetData|AbilityTargetDatafromActor (Variables|Default|GetOwningWeapon)))
              (Ability|EndAbility)
              (else
                (Ability|EndAbility)))))))
    (:CastFailed
      (Development|PrintString "GA_Artillery2 - Cast to Player Mech Failed")
      (Ability|EndAbility))))