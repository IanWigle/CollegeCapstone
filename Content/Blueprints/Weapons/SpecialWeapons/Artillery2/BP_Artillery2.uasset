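; Artillery2 special weapon Blueprint that sets up its Gameplay Ability System state on spawn.
; BeginPlay initializes the weapon ability system's base attribute set from the Artillery2 data table, then applies an artillery tags gameplay effect to itself.
; The construction script makes the skeletal mesh always tick pose and refresh bones regardless of visibility.
; An unconnected debug branch for printing an attribute value never runs.
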(event EventBeginPlay
  (bind _m_weaponabilitysystemcomponent (Variables|Default|Getm_WeaponAbilitySystemComponent))
  (Class|AbilitySystemComponent|InitStats _m_weaponabilitysystemcomponent "/Script/Outpost_Production.BaseWeaponAttributeSet" "/Game/Blueprints/Weapons/SpecialWeapons/Artillery2/Artillery2DataTable.Artillery2DataTable")
  (GameplayEffects|ApplyGameplayEffectToSelf :self _m_weaponabilitysystemcomponent :GameplayEffectClass "/Game/Blueprints/Weapons/SpecialWeapons/Artillery2/GE_Artillery_Tags.GE_Artillery_Tags_C"))

(event EventTick
  (params (DeltaSeconds :type Float%20%28single-precision%29)))

(fn ConstructionScript
  (Variables|/Script/Engine.SkinnedMeshComponent|SetVisibilityBasedAnimTickOption (Variables|Default|GetSkeletalMeshComponent) "AlwaysTickPoseAndRefreshBones"))