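; Gameplay ability that fires the mech's Gauss Cannon, a wide shot that can hit multiple enemies.
; It ends early if the weapon is reloading, otherwise it multicasts fire and sphere-traces along the player's camera, with debug drawing on.
; Enemy-tagged hits get a multicast impact and SetByCaller GE_Damage, then GE_Reload is applied to the weapon and the ability ends.
; Failed weapon or mech casts only print, without ending the ability.
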(event Ability|EventActivateAbility
  (bind _asbase_weapon (Utilities|Casting|CastToBaseWeapon (Ability|GetAvatarActorfromActorInfo))
    (:then
      (Variables|Default|SetWeapon _asbase_weapon)
      (bind _asplayer_mech (Utilities|Casting|CastToPlayerMech (Ability|GetOwningActorfromActorInfo))
        (:then
          (Variables|Default|SetPlayer _asplayer_mech)
          (if (GameplayTags|HasAnyMatchingGameplayTags (Ability|GetAbilitySystemComponent (Variables|Default|GetWeapon)) (GameplayTags|MakeGameplayTagContainerfromArray (Utilities|Array|MakeArray (GameplayTags|MakeLiteralGameplayTag "(TagName=\"Weapon.Reloading\")"))))
            (Ability|EndAbility)
            (else
              (Class|BaseWeapon|NetMulticastWeaponFireStarted (Variables|Default|GetWeapon))
              (bind _outhits (Collision|MultiSphereTraceByChannel (Transformation|GetWorldLocation (Variables|/Script/Outpost_Production.PlayerMech|Getm_FollowCamera _asplayer_mech)) (+ (Transformation|GetWorldLocation (Variables|/Script/Outpost_Production.PlayerMech|Getm_FollowCamera _asplayer_mech)) (* (Math|Vector|GetForwardVector (Variables|/Script/Outpost_Production.PlayerMech|Getm_FollowCamera _asplayer_mech)) (Math|Conversions|ToVector(Float) (.ReturnValue (Ability|Attribute|GetFloatAttribute (Variables|Default|GetWeapon) "(AttributeName=\"\",Attribute=StructProperty'\"/Script/Outpost_Production.BaseWeaponAttributeSet:m_HardRange\"',AttributeOwner=None)"))))) 1e+02 "TraceTypeQuery4" false (Utilities|Array|MakeArray (Variables|Default|GetWeapon) (Variables|Default|GetPlayer)) "ForDuration"))
              (for _array_element _outhits
                (Utilities|IsValid (.HitActor (Collision|BreakHitResult _array_element))
                  (:Is%20Valid
                    (if (Actor|ActorHasTag (.HitActor (Collision|BreakHitResult _array_element)) "Enemy")
                      (Class|BaseWeapon|NetMulticastWeaponHit (Variables|Default|GetWeapon) (.ImpactPoint (Collision|BreakHitResult _array_element)) (.HitActor (Collision|BreakHitResult _array_element)))
                      (bind _returnvalue (Ability|GameplayEffect|AssignTagSetbyCallerMagnitude (Ability|MakeOutgoingGameplayEffectSpec "/Game/Blueprints/Weapons/GE_Damage.GE_Damage_C") "(TagName=\"Damage\")" (* (.ReturnValue (Ability|Attribute|GetFloatAttribute (Variables|Default|GetWeapon) "(AttributeName=\"\",Attribute=StructProperty'\"/Script/Outpost_Production.BaseWeaponAttributeSet:m_Damage\"',AttributeOwner=None)")) -1.0)))
                      (GameplayEffects|ApplyGameplayEffectSpecToTarget _returnvalue (Ability|TargetData|AbilityTargetDatafromHitResult _array_element))))))
              (bind _returnvalue_2 (Ability|GameplayEffect|AssignTagSetbyCallerMagnitude (Ability|MakeOutgoingGameplayEffectSpec "/Game/Blueprints/Weapons/MainWeapons/GE_Reload.GE_Reload_C") "(TagName=\"Weapon.Reloading\")" (.ReturnValue (Ability|Attribute|GetFloatAttribute (Variables|Default|GetWeapon) "(AttributeName=\"\",Attribute=StructProperty'\"/Script/Outpost_Production.BaseWeaponAttributeSet:m_ReloadSpeed\"',AttributeOwner=None)"))))
              (GameplayEffects|ApplyGameplayEffectSpecToTarget _returnvalue_2 (Ability|TargetData|AbilityTargetDatafromActor (Variables|Default|GetWeapon)))
              (Ability|EndAbility))))
        (:CastFailed
          (Development|PrintString "GAGaussCannon: owner is not a playermech"))))
    (:CastFailed
      (Development|PrintString "GAGaussCannon: cast to baseweapon failed"))))