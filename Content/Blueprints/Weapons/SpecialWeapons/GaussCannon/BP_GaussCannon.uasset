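; Gauss Cannon special weapon for player mechs, handling its ability system setup and firing effects.
; On BeginPlay it initializes the weapon attribute set from the Gauss Cannon data table and applies its tags gameplay effect.
; Firing activates the attack particle system, passes the owning mech's follow-camera forward vector as its direction parameter, and plays audio.
; A non-player-mech owner only triggers a debug message.
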(event EventBeginPlay
  (bind _m_weaponabilitysystemcomponent (Variables|Default|Getm_WeaponAbilitySystemComponent))
  (Class|AbilitySystemComponent|InitStats _m_weaponabilitysystemcomponent "/Script/Outpost_Production.BaseWeaponAttributeSet" "/Game/Blueprints/Weapons/SpecialWeapons/GaussCannon/GaussCannonDataTable.GaussCannonDataTable")
  (GameplayEffects|ApplyGameplayEffectToSelf :self _m_weaponabilitysystemcomponent :GameplayEffectClass "/Game/Blueprints/Weapons/SpecialWeapons/GaussCannon/GE_GaussCannon_Tags.GE_GaussCannon_Tags_C"))

(event EventWeaponFireEvent
  (bind _attacksystem (Variables|Default|GetAttackSystem))
  (bind _asplayer_mech (Utilities|Casting|CastToPlayerMech (Components|GetOwner))
    (:then
      (Components|Activation|Activate _attacksystem true)
      (Effects|Components|ParticleSystem|SetVectorParameter _attacksystem "User.Direction" (Math|Vector|GetForwardVector (Variables|/Script/Outpost_Production.PlayerMech|Getm_FollowCamera _asplayer_mech)))
      (Audio|Components|Audio|Play (Variables|Default|Getm_AudioComponent) 0.0))
    (:CastFailed
      (Development|PrintString "BP_GaussCannon: Owner is not a player mech"))))

(fn ConstructionScript)