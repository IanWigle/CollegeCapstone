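; Base Blueprint for flora props that glow in response to actors nearby.
; On BeginPlay it creates dynamic material instances for three leaf slots and a bark slot on the flora mesh.
; Proximity enter and leave events share one update that scales each material's Emission with the count of entered actors, guarded only by a validity check on the first leaf material.
; The construction script and Scaler replication callback are empty.
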(event EventBeginPlay
  (bind _returnvalue (Rendering|Material|CreateDynamicMaterialInstance (Variables|Default|Getm_FloraMesh) 0 "/Game/Assets/3D_Assets/Level/Flora/BeaconTree/M_Leaf1.M_Leaf1" "None" :!class /Script/Engine.PrimitiveComponent))
  (Variables|Default|SetLeaf1Shader _returnvalue)
  (bind _returnvalue_2 (Rendering|Material|CreateDynamicMaterialInstance (Variables|Default|Getm_FloraMesh) 1 "/Game/Assets/3D_Assets/Level/Flora/BeaconTree/M_Leaf2.M_Leaf2" "None" :!class /Script/Engine.PrimitiveComponent))
  (Variables|Default|SetLeaf2Shader _returnvalue_2)
  (bind _returnvalue_3 (Rendering|Material|CreateDynamicMaterialInstance (Variables|Default|Getm_FloraMesh) 2 "/Game/Assets/3D_Assets/Level/Flora/BeaconTree/M_Leaf3.M_Leaf3" "None" :!class /Script/Engine.PrimitiveComponent))
  (Variables|Default|SetLeaf3Shader _returnvalue_3)
  (bind _returnvalue_4 (Rendering|Material|CreateDynamicMaterialInstance (Variables|Default|Getm_FloraMesh) 3 "/Game/Assets/3D_Assets/Level/Flora/BeaconTree/M_Bark.M_Bark" "None" :!class /Script/Engine.PrimitiveComponent))
  (Variables|Default|SetBarkShader _returnvalue_4))

(event Collision|EventActorBeginOverlap
  (params (OtherActor :type Actor%20Object%20Reference)))

(event EventTick
  (params (DeltaSeconds :type Float%20%28single-precision%29)))

(event EventActorEntersProximity
  (params (actor :type Actor%20Object%20Reference))
  (bind _leaf1shader (Variables|Default|GetLeaf1Shader))
  (bind _m_enteredactors (Variables|Default|Getm_EnteredActors))
  (bind _returnvalue (Utilities|Array|Length _m_enteredactors))
  (bind _returnvalue_2 (* _returnvalue 3))
  (bind _returnvalue_3 (Math|Conversions|ToFloat(Integer) _returnvalue_2))
  (Utilities|IsValid _leaf1shader
    (:Is%20Valid
      (Rendering|Material|SetScalarParameterValue _leaf1shader "Emission" _returnvalue_3 :!class /Script/Engine.MaterialInstanceDynamic)
      (Rendering|Material|SetScalarParameterValue (Variables|Default|GetLeaf2Shader) "Emission" _returnvalue_3 :!class /Script/Engine.MaterialInstanceDynamic)
      (Rendering|Material|SetScalarParameterValue (Variables|Default|GetLeaf3Shader) "Emission" _returnvalue_3 :!class /Script/Engine.MaterialInstanceDynamic)
      (Rendering|Material|SetScalarParameterValue (Variables|Default|GetBarkShader) "Emission" _returnvalue_3 :!class /Script/Engine.MaterialInstanceDynamic))))

(event EventActorLeavesProximity
  (params (actor :type Actor%20Object%20Reference))
  (bind _leaf1shader (Variables|Default|GetLeaf1Shader))
  (bind _m_enteredactors (Variables|Default|Getm_EnteredActors))
  (bind _returnvalue (Utilities|Array|Length _m_enteredactors))
  (bind _returnvalue_2 (* _returnvalue 3))
  (bind _returnvalue_3 (Math|Conversions|ToFloat(Integer) _returnvalue_2))
  (Utilities|IsValid _leaf1shader
    (:Is%20Valid
      (Rendering|Material|SetScalarParameterValue _leaf1shader "Emission" _returnvalue_3 :!class /Script/Engine.MaterialInstanceDynamic)
      (Rendering|Material|SetScalarParameterValue (Variables|Default|GetLeaf2Shader) "Emission" _returnvalue_3 :!class /Script/Engine.MaterialInstanceDynamic)
      (Rendering|Material|SetScalarParameterValue (Variables|Default|GetLeaf3Shader) "Emission" _returnvalue_3 :!class /Script/Engine.MaterialInstanceDynamic)
      (Rendering|Material|SetScalarParameterValue (Variables|Default|GetBarkShader) "Emission" _returnvalue_3 :!class /Script/Engine.MaterialInstanceDynamic))))

(fn ConstructionScript)

(fn OnRepScaler)